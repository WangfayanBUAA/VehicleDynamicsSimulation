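; BP_SurfaceTest is a test actor that follows the height of BP_WaterSurface actors.
; It caches all water surfaces on BeginPlay, then each Tick sets its Z to each one's GetWaterHeightAtLocation at its XY, so the last in the list wins.
; Downward visibility traces run on Tick and in the construction script (with debug drawing in the latter), but their results are unused.
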(event EventBeginPlay
  (bind _outactors (Actor|GetAllActorsOfClass "/Game/WaterSystem/BluePrint/BP_WaterSurface.BP_WaterSurface_C"))
  (Variables|Default|SetWaterList _outactors))

(event Collision|EventActorBeginOverlap
  (params (OtherActor :type Actor%20Object%20Reference)))

(event EventTick
  (params (DeltaSeconds :type Float%20%28single-precision%29))
  (bind _self self)
  (bind _self_2 self)
  (bind _returnvalue (Transformation|GetActorLocation _self))
  (bind _returnvalue_2 (Transformation|GetActorLocation _self_2))
  (bind (_x _y) (Math|Vector|BreakVector _returnvalue_2))
  (Collision|LineTraceByChannel _returnvalue (+ _returnvalue "0, 0,-100.000000") "TraceTypeQuery1" false 0 "None")
  (for _array_element (Variables|Default|GetWaterList)
    (Transformation|SetActorLocation (Math|Vector|MakeVector _x _y (Default|GetWaterHeightatLocation _array_element (Math|Conversions|ToVector2D(Vector) _returnvalue_2))) false false)))

(fn ConstructionScript
  (bind _self self)
  (bind _returnvalue (Transformation|GetActorLocation _self))
  (Collision|LineTraceByChannel _returnvalue (+ _returnvalue "0, 0,-100.000000") "TraceTypeQuery1" false 0 "ForDuration"))