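; Base water wave Blueprint that adds a directional sine wave to a parent water surface and answers height queries at a location.
; InitWave stores the wave settings and passes them to a material instance created by the parent surface.
; UpdateHeightMap advances time and has the parent draw that material to the surface.
; GetHeightAtLocation computes height on the CPU, projecting the location onto the wave direction with a sinusoidal phase warp.
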(fn UpdateHeightMap
  (params (deltaSeconds :type Float%20%28single-precision%29))
  (Utilities|FlowControl|Sequence
    (:then_0
      ;[1 1 1] Comment
      (Variables|Default|SettimeStep (+ deltaSeconds (Variables|Default|GettimeStep)))
      (return (Variables|Default|GettimeStep)))
    (:then_1
      (Rendering|Material|SetScalarParameterValue (Variables|Default|GetMT_WaveGenerator) "Time" (Variables|Default|GettimeStep) :!class /Script/Engine.MaterialInstanceDynamic))
    (:then_2
      (Default|DrawWavetoSurface (Variables|Default|GetParent%20Water%20Surface) (Variables|Default|GetMT_WaveGenerator)))))

(fn GetHeightatLocation
  (params (inWorldLocation :type Vector%202D%20Structure))
  (bind _output_get (LocalVariables|SetWorldLocation inWorldLocation))
  (bind _returnvalue (BaseSignals|SinWaveSignal (utils|GetSignalPosition _output_get) (Variables|Default|GetwaveLength)))
  (return (* _returnvalue (Variables|Default|GetWaterWaveHeight))))

(fn InitWave
  (params (ParentWaterSurface :type BP%20Water%20Surface%20Object%20Reference) (inWaterOriginUV :type Vector%202D%20Structure) (inWaterSize :type Vector%202D%20Structure) (WaterWaveHeightSize :type Float%20%28single-precision%29) (inWaveDirection :type Vector%202D%20Structure) (inWaveLength :type Float%20%28single-precision%29) (inWaveSpeed :type Float%20%28single-precision%29))
  (Utilities|FlowControl|Sequence
    (:then_0
      (bind _output_get (Variables|Default|SetWaterWaveHeight WaterWaveHeightSize))
      (Variables|Default|SetwaveMaterialHeight _output_get)
      (Variables|Default|SetwaveDirection inWaveDirection)
      (Variables|Default|SetwaveLength inWaveLength)
      (Variables|Default|SetwaveSpeed inWaveSpeed))
    (:then_1
      (Utilities|FlowControl|Sequence
        (:then_0
          (Variables|Default|SetParent%20Water%20Surface ParentWaterSurface)
          (LocalVariables|SetWaterOriginUV inWaterOriginUV)
          (LocalVariables|SetWaterSize inWaterSize))
        (:then_1
          (bind _returnvalue (Default|CreateNatureWaveMaterial (Variables|Default|GetParent%20Water%20Surface) (Variables|Default|GetWaveMaterialType)))
          (Variables|Default|SetMT_WaveGenerator _returnvalue)
          (Rendering|Material|SetScalarParameterValue (Variables|Default|GetMT_WaveGenerator) "waveHeight" (Variables|Default|GetwaveMaterialHeight) :!class /Script/Engine.MaterialInstanceDynamic)
          (Rendering|Material|SetScalarParameterValue (Variables|Default|GetMT_WaveGenerator) "waveLength" (Variables|Default|GetwaveLength) :!class /Script/Engine.MaterialInstanceDynamic)
          (Rendering|Material|SetScalarParameterValue (Variables|Default|GetMT_WaveGenerator) "waveSpeed" (Variables|Default|GetwaveSpeed) :!class /Script/Engine.MaterialInstanceDynamic)
          (Rendering|Material|SetVectorParameterValue (Variables|Default|GetMT_WaveGenerator) "WaterOriginUV" (Math|Color|MakeColor (.x (LocalVariables|GetWaterOriginUV)) (.y (LocalVariables|GetWaterOriginUV)) 0.0) :!class /Script/Engine.MaterialInstanceDynamic)
          (Rendering|Material|SetVectorParameterValue (Variables|Default|GetMT_WaveGenerator) "WaterSize" (Utilities|Struct|MakeLinearColor (.x (LocalVariables|GetWaterSize)) (.y (LocalVariables|GetWaterSize)) 0.0 1.0) :!class /Script/Engine.MaterialInstanceDynamic)
          (Rendering|Material|SetVectorParameterValue (Variables|Default|GetMT_WaveGenerator) "Direction" (Utilities|Struct|MakeLinearColor (.X (Math|Vector2D|BreakVector2D (Variables|Default|GetwaveDirection))) (.Y (Math|Vector2D|BreakVector2D (Variables|Default|GetwaveDirection))) 0.0 1.0) :!class /Script/Engine.MaterialInstanceDynamic))))))

(fn SinWaveSignal
  (params (inPoint :type Vector%202D%20Structure) (inWaveLength :type Float%20%28single-precision%29))
  (return (* (+ (Math|Trig|Sin(Radians) (* (/ (.X (Math|Vector2D|BreakVector2D inPoint)) inWaveLength) (Math|Trig|GetPI) 2.0)) 1.0) 0.5)))

(fn GetSignalPosition
  (params (inLocation :type Vector%202D%20Structure))
  (LocalVariables|SetLocationInWater inLocation)
  (Utilities|FlowControl|Sequence
    (:then_0
      (bind _output_get (LocalVariables|SettmpDirection (Math|Vector2D|Normalize2D (Variables|Default|GetwaveDirection))))
      (LocalVariables|Setx (+ (Math|Vector2D|DotProduct(2D) _output_get (LocalVariables|GetLocationInWater)) (* (Variables|Default|GettimeStep) (Variables|Default|GetwaveSpeed)))))
    (:then_1
      (bind _output_get_2 (LocalVariables|Settmp%20N%20Direction (Math|Vector2D|MakeVector2D (* (.y (LocalVariables|GettmpDirection)) -1.0) (.x (LocalVariables|GettmpDirection)))))
      (LocalVariables|SetY (Math|Vector2D|DotProduct(2D) _output_get_2 (LocalVariables|GetLocationInWater))))
    (:then_3
      (return (Math|Vector2D|MakeVector2D (+ (/ (* (Math|Trig|Sin(Radians) (/ (+ (LocalVariables|Getx) (LocalVariables|GetY)) 2e+04)) (Variables|Default|GetwaveLength)) 1.0) (LocalVariables|Getx)) (LocalVariables|GetY))))))