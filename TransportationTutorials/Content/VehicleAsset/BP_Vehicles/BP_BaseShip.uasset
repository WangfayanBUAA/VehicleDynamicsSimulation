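; Base physics ship that adapts a parent vehicle class to water, driven by buoyancy, propeller and rudder components gathered at construction.
; Buoyancy components linked to the level's water surface push the hull vertically, while propellers add thrust that tapers near max speed.
; Rudders and hull apply capped side-friction forces from point velocity, with each rudder adding a counter-force ahead to turn the ship.
; It also spins propellers and exposes a capture image of its water shape.
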(event EventBeginPlay
  (CallFunction|InitVehicle)
  (bind _returnvalue (Actor|GetActorOfClass "/Game/WaterSystem/BluePrint/BP_WaterSurface.BP_WaterSurface_C"))
  (Variables|Default|SetWaterSurface _returnvalue)
  (for _array_element (Variables|Default|GetBuoyancyList)
    (Default|InitBuoyancy _array_element (Variables|Default|GetWaterSurface))))

(event Collision|EventActorBeginOverlap
  (params (OtherActor :type Actor%20Object%20Reference)))

(event EventTick
  (params (DeltaSeconds :type Float%20%28single-precision%29))
  (|CallParentFunction DeltaSeconds) ; This node is disabled and will not be called.\nDrag off pins to build functionality.
)

(fn ConstructionScript
  (Variables|Default|SetBuoyancyList (Actor|GetComponentsByClass "/Game/VehicleAsset/BP_Vehicles/Components/BP_buoyancy.BP_buoyancy_C"))
  (Variables|Default|SetPropellerList (Actor|GetComponentsByClass "/Game/VehicleAsset/BP_Vehicles/Components/BPC_Propeller.BPC_Propeller_C"))
  (Variables|Default|SetRudderList (Actor|GetComponentsByClass "/Game/VehicleAsset/BP_Vehicles/Components/BP_ShipRudder.BP_ShipRudder_C")))

(fn UpdateSupportForce
  (for _array_element (Variables|Default|GetBuoyancyList)
    (bind _output_get (LocalVariables|SettmpBuoyancy _array_element))
    (Class|PrimitiveComponent|AddForceatLocation (Variables|Default|GetVehicleBody) (* (* (.ForceVector (Default|GetSupportVector _output_get (Variables|Default|GetDeltaSeconds))) (.SupportForce (Default|GetSupportVector _output_get (Variables|Default|GetDeltaSeconds)))) "0, 0,1.000000") (Transformation|GetWorldLocation (LocalVariables|GettmpBuoyancy)) "None")))

(fn UpdateTractionForce
  (if (Variables|Default|GetisEngineStart)
    (Utilities|FlowControl|Sequence
      (:then_0
        (for _array_element (Variables|Default|GetPropellerList)
          (bind _output_get (LocalVariables|SettmpPropeller _array_element))
          (bind _force (Default|UpdatePropellForce _output_get (Variables|Default|GetDeltaSeconds) (* (+ (* (Variables|Default|GetPowerValue) (Math|Conversions|ToFloat(Integer) (Variables|Default|GetGearDirection))) (LocalVariables|GetAdjustPower)) 1.0 (- 1.0 (Math|Float|Clamp(Float) (/ (- (CallFunction|GetSpeed) (- (Variables|Default|GetMaxSpeed) 3.0)) 5.0))))))
          (Class|PrimitiveComponent|AddForceatLocation (Variables|Default|GetVehicleBody) _force (Transformation|GetWorldLocation (LocalVariables|GettmpPropeller)) "None")))
      (:then_1
        (bind (_output_get_2 _outshipdirection) (CallFunction|GetSideFrictionForce (Transformation|GetWorldTransform (Variables|Default|GetVehicleBody))))
        (LocalVariables|SetSteerForce _output_get_2)
        (LocalVariables|SetShipDirection _outshipdirection)
        (Class|PrimitiveComponent|AddForceatLocation (Variables|Default|GetVehicleBody) (* (LocalVariables|GetSteerForce) 3e+01) (Transformation|GetWorldLocation (Variables|Default|GetVehicleBody)) "None")))))

(fn UpdateLandShapeInput
  (for _array_element (Variables|Default|GetBuoyancyList)
    (Default|UpdateSuspensionLength _array_element 0.0)))

(fn InitVehicle
  (bind _output_get (Variables|Default|SetvehicleMass (Physics|GetMass (Variables|Default|GetVehicleBody))))
  (LocalVariables|SettmpMass (/ _output_get 1e+02))
  (Variables|Default|SetMaxBreakForce (* (LocalVariables|GettmpMass) (Variables|Default|GetMaxBreakForce) 5.0))
  (Variables|Default|SetBreakSpeed (* (LocalVariables|GettmpMass) (Variables|Default|GetBreakSpeed) 5.0))
  (Variables|Default|SetMaxPower (* (LocalVariables|GettmpMass) (Variables|Default|GetMaxPower)))
  (Variables|Default|SetPowerUpSpeed (* (LocalVariables|GettmpMass) (Variables|Default|GetPowerUpSpeed) 1.5))
  (Variables|Default|SetSuspensionDamp (* (LocalVariables|GettmpMass) (Variables|Default|GetSuspensionDamp) 1.5))
  (Variables|Default|SetSuspensionStrength (* (Variables|Default|GetSuspensionStrength) (LocalVariables|GettmpMass) 2e+01))
  (for _array_element (Variables|Default|GetBuoyancyList)
    (Variables|/Game/VehicleAsset/BP_Vehicles/Components/BP_VehicleWheel.BP_VehicleWheel_C|SetSuspensonDamp _array_element (Variables|Default|GetSuspensionDamp))
    (Variables|/Game/VehicleAsset/BP_Vehicles/Components/BP_VehicleWheel.BP_VehicleWheel_C|SetSuspStrength _array_element (Variables|Default|GetSuspensionStrength))))

(fn UpdateSteeringForce
  ;[1 1 1] 循环便利悬挂系统
  (for _array_element (Variables|Default|GetRudderList)
    (LocalVariables|SetCurrentRudder _array_element)
    (bind (_output_get _outshipdirection) (CallFunction|GetSideFrictionForce (Transformation|GetWorldTransform (LocalVariables|GetCurrentRudder))))
    (LocalVariables|SetSteerForce _output_get)
    (LocalVariables|SetShipDirection _outshipdirection)
    (Class|PrimitiveComponent|AddForceatLocation (Variables|Default|GetVehicleBody) (LocalVariables|GetSteerForce) (.location (Transformation|GetWorldTransform (LocalVariables|GetCurrentRudder))) "None")
    (Class|PrimitiveComponent|AddForceatLocation (Variables|Default|GetVehicleBody) (* (LocalVariables|GetSteerForce) -1.0) (+ (Transformation|GetWorldLocation (Variables|Default|GetVehicleBody)) (* (LocalVariables|GetShipDirection) 1e+03)) "None")))

(fn UpdateWheelYaw
  (for _array_element (Variables|Default|GetRudderList)
    (bind _output_get (LocalVariables|SettmpRudder _array_element))
    (Default|SetRudderSteerAngle _output_get (* -1 (Variables|Default|GetSteeringAngle)))))

(fn GetSideFrictionForce
  (params (InTransform :type Transform))
  (bind _vehiclebody (Variables|Default|GetVehicleBody))
  (bind _returnvalue (Physics|GetMass _vehiclebody))
  (LocalVariables|SetTmpTransform InTransform)
  ;[1 1 1] 悬挂接触面法线
  (LocalVariables|SetnormalVector (Math|Vector|GetUpVector (.rotation (LocalVariables|GetTmpTransform))))
  (Utilities|FlowControl|Sequence
    (:then_0
      ;[1 1 1] 车轮组件的实际速度
      (bind _returnvalue_2 (Class|PrimitiveComponent|GetPhysicsLinearVelocityatPoint (Variables|Default|GetVehicleBody) (.location (LocalVariables|GetTmpTransform)) "None"))
      (LocalVariables|SetrealVelocityDirection (Math|Vector|Normalize _returnvalue_2))
      (LocalVariables|SetrealSpeed (Math|Vector|VectorLength _returnvalue_2))
      (LocalVariables|SetShipDirection (Math|Vector|GetForwardVector (Transformation|GetWorldRotation (Variables|Default|GetVehicleBody)))))
    (:then_1
      ;[1 1 1] 悬挂右侧向量
      (LocalVariables|SettargetDirection (Math|Rotator|GetRotationXVector (.rotation (LocalVariables|GetTmpTransform))))
      (LocalVariables|SetHDirection (Math|Vector|GetRightVector (.rotation (LocalVariables|GetTmpTransform)))))
    (:then_2
      ;[1 1 1] 获取侧向转向阻力
      (bind _output_get (LocalVariables|SetdeltaVelocity (* (- (LocalVariables|GettargetDirection) (LocalVariables|GetrealVelocityDirection)) (LocalVariables|GetrealSpeed))))
      (LocalVariables|SettargetCentripetalAcceleration (* (LocalVariables|GetHDirection) (Math|Vector|DotProduct (LocalVariables|GetHDirection) (CallFunction|ProjecttoPlane (LocalVariables|GetnormalVector) _output_get)))))
    (:then_4
      (bind _output_get_2 (LocalVariables|SetSteerForce (* (Math|Vector|Normalize (* (LocalVariables|GettargetCentripetalAcceleration) _returnvalue)) (Math|Float|Min(Float) (Math|Vector|VectorLength (* (LocalVariables|GettargetCentripetalAcceleration) _returnvalue)) (* (Variables|Default|GetFrictionRate) _returnvalue)))))
      (return _output_get_2 (LocalVariables|GetShipDirection)))))

(fn UpdateVehicleMovement
  (params (inDeltaSeconds :type Float%20%28single-precision%29))
  (bind _returnvalue (CallFunction|GetSpeed))
  (bind _maxspeed (Variables|Default|GetMaxSpeed))
  (bind _geardirection (Variables|Default|GetGearDirection))
  (bind _returnvalue_2 (/ _returnvalue _maxspeed))
  (bind _output_get (LocalVariables|SetDS inDeltaSeconds))
  (|CallParentFunction _output_get)
  (for _array_element (Variables|Default|GetPropellerList)
    (Default|PropellerRot _array_element (LocalVariables|GetDS) (* (Math|Integer|SelectInt _geardirection (Math|Float|Truncate (Math|Float|Sign(Float) _returnvalue_2)) (!= _geardirection 0)) (Math|Float|Max(Float) (/ (Variables|Default|GetPowerValue) (Variables|Default|GetMaxPower)) _returnvalue_2)))))

(fn GetSpeed
  (bind _vehiclebody (Variables|Default|GetVehicleBody))
  (return (* (Math|Vector|DotProduct (Transformation|GetComponentVelocity _vehiclebody) (Math|Vector|GetForwardVector (Transformation|GetWorldRotation _vehiclebody))) 0.036)))

(fn CaptureWaterShape
  (return "/Game/VehicleAsset/Mesh/West_Ship_DDG102/ShipCapture.ShipCapture" (Variables|/Script/Engine.SceneCaptureComponent2D|GetOrthoWidth (Variables|Default|GetSceneCaptureComponent2D))))