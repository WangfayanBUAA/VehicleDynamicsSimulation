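; BP_VehicleController is a controller that lets the player cycle through the vehicles placed in the level and shows a speed HUD.
; On BeginPlay it gathers every BP_BaseVehiclePawn, possesses the one at the current index and adds a Widget_SpeedUI to the viewport.
; The ChangeVehicle input possesses the next pawn, wrapping around the list.
; Each tick it passes the HUD widget to the possessed vehicle's UpdateHUD.
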(event EventBeginPlay
  (Utilities|FlowControl|Sequence
    (:then_0
      (bind _outactors (Actor|GetAllActorsOfClass "/Game/VehicleAsset/BP_Vehicles/BP_BaseVehiclePawn.BP_BaseVehiclePawn_C"))
      (Variables|Default|SetVehicleList _outactors)
      (bind _output_get (Variables|Default|SetCurrentVehicle (Utilities|Array|Get(acopy) (Variables|Default|GetVehicleList) (Variables|Default|GetVehicleIndex))))
      (Pawn|Possess _output_get))
    (:then_1
      (bind _returnvalue (UserInterface|CreateWidget "/Game/VehicleAsset/widget/Widget_SpeedUI.Widget_SpeedUI_C" (Game|GetPlayerController 0)))
      (bind _output_get_2 (Variables|Default|SetVehicleHUD _returnvalue))
      (UserInterface|Viewport|AddtoViewport _output_get_2 0))))

(event EventTick
  (params (DeltaSeconds :type Float%20%28single-precision%29))
  (Default|UpdateHUD (Variables|Default|GetCurrentVehicle) (Variables|Default|GetVehicleHUD)))

(event Input|ActionEvents|InputActionChangeVehicle
  (params (Key :type Key%20Structure))
  (:Pressed
    (Variables|Default|SetVehicleIndex (Math|Integer|%(Integer) (+ (Variables|Default|GetVehicleIndex) 1) (Utilities|Array|Length (Variables|Default|GetVehicleList))))
    (bind _output_get (Variables|Default|SetCurrentVehicle (Utilities|Array|Get(acopy) (Variables|Default|GetVehicleList) (Variables|Default|GetVehicleIndex))))
    (Pawn|Possess _output_get)))

(fn ConstructionScript)