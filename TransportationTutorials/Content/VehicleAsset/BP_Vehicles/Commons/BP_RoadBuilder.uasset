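; Road builder actor that lays spline mesh segments along an editable spline at construction time, optionally conforming to the terrain.
; LayoutMeshOnLand splits the spline at a fixed interval and uses FindLandPoint's vertical line traces to place each segment.
; Optional normal matching banks segments through GetRollingAtPoint, averaging three normals and carrying roll forward for continuity.
; Both road ends sink into the ground, and every segment receives scale, material and blocking collision.
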(event EventBeginPlay)

(event Collision|EventActorBeginOverlap
  (params (OtherActor :type Actor%20Object%20Reference)))

(fn ConstructionScript
  (Variables|Default|SetRefresh false)
  (Components|StaticMesh|SetStaticMesh (Variables|Default|GetFenceMeshComp) (Variables|Fence|GetFence%20Mesh))
  (Utilities|FlowControl|Sequence
    (:then_0
      (CallFunction|LayoutMeshonLand))))

(fn FindLandPoint
  (params (inSpline :type Spline%20Component%20Object%20Reference) (positionInLine :type Float%20%28single-precision%29) (inNeedMatchLand :type Boolean) (RigthOffset :type Float%20%28single-precision%29))
  (bind _returnvalue (Spline|GetLocationatDistanceAlongSpline inSpline positionInLine "Local"))
  (bind _returnvalue_2 (Spline|GetLocationatDistanceAlongSpline inSpline positionInLine "Local"))
  (bind _returnvalue_3 (Spline|GetLocationatDistanceAlongSpline inSpline positionInLine "World"))
  (bind _returnvalue_4 (Class|SplineComponent|GetRightVectoratDistanceAlongSpline inSpline positionInLine "World"))
  (bind _returnvalue_5 (* _returnvalue_4 RigthOffset))
  (bind _returnvalue_6 (+ _returnvalue_3 _returnvalue_5))
  (if inNeedMatchLand
    (bind (_outhit _returnvalue_7) (Collision|LineTraceForObjects (+ _returnvalue_6 "0, 0,10000.000000") (+ _returnvalue_6 "0, 0,-10000.000000") (LocalVariables|GetNewLocalVar_1) false 0 "None"))
    (if _returnvalue_7
      (bind _output_get (LocalVariables|SetLandLocation (.Location (Collision|BreakHitResult _outhit))))
      (return (Math|Transform|InverseTransformLocation (Transformation|GetWorldTransform inSpline) _output_get) _output_get (.ImpactNormal (Collision|BreakHitResult _outhit)))
      (else
        (return _returnvalue (Math|Transform|TransformLocation (Transformation|GetWorldTransform inSpline) _returnvalue) "0, 0, 0")))
    (else
      (return _returnvalue_2 (Math|Transform|TransformLocation (Transformation|GetWorldTransform inSpline) _returnvalue_2) "0, 0, 0"))))

(fn GetRollingatPoint
  (params (tanInSpline :type Vector) (LandNormal :type Vector))
  (bind (_x _y) (Math|Vector|BreakVector tanInSpline))
  (LocalVariables|SetXInBody (Math|Vector|Normalize tanInSpline))
  (bind _output_get (LocalVariables|SetYInBody (Math|Vector|Normalize (Math|Vector|MakeVector _y (* _x -1.0) 0.0))))
  (bind _output_get_2 (LocalVariables|SetZInBody (Math|Vector|Normalize (Math|Vector|CrossProduct _output_get (LocalVariables|GetXInBody)))))
  (return (* (Class|KismetMathLibrary|DegAcos (Math|Vector|DotProduct _output_get_2 LandNormal)) (Math|Float|SelectFloat 1.0 -1.0 (>= (Math|Vector|DotProduct LandNormal (LocalVariables|GetYInBody)) 0.0))) _output_get_2))

(fn LayoutMeshonLand
  (bind _tmpfenceindex (LocalVariables|GettmpFenceIndex))
  (bind _mainmeshinterval (Variables|Default|GetMainMeshInterval))
  (bind _spline (Variables|Default|GetSpline))
  (bind _needmatchland (Variables|Default|GetNeedMatchLand))
  (bind _spline_2 (Variables|Default|GetSpline))
  (bind _mainmeshinterval_2 (Variables|Default|GetMainMeshInterval))
  (bind _mainmeshinterval_3 (Variables|Default|GetMainMeshInterval))
  (bind _tmpfenceindex_2 (LocalVariables|GettmpFenceIndex))
  (bind _spline_3 (Variables|Default|GetSpline))
  (bind _meshsize (Variables|Default|GetMeshSIze))
  (bind _spline_4 (Variables|Default|GetSpline))
  (bind _mainmeshinterval_4 (Variables|Default|GetMainMeshInterval))
  (bind _needmatchland_2 (Variables|Default|GetNeedMatchLand))
  (bind _tmpfenceindex_3 (LocalVariables|GettmpFenceIndex))
  (bind _spline_5 (Variables|Default|GetSpline))
  (bind _roadoffset (Variables|Default|GetRoadOffset))
  (bind _mainmeshinterval_5 (Variables|Default|GetMainMeshInterval))
  (bind _returnvalue (Math|Conversions|ToFloat(Integer) _tmpfenceindex))
  (bind _returnvalue_2 (Math|Conversions|ToFloat(Integer) _tmpfenceindex_2))
  (bind _returnvalue_3 (Math|Vector2D|MakeVector2D (.y _meshsize) (.z _meshsize)))
  (bind _returnvalue_4 (Math|Conversions|ToFloat(Integer) _tmpfenceindex_3))
  (bind _returnvalue_5 (+ _returnvalue 0.0))
  (bind _returnvalue_6 (+ _returnvalue 1.0))
  (bind _returnvalue_7 (+ _returnvalue_4 0.0))
  (bind _returnvalue_8 (+ _returnvalue_4 1.0))
  (bind _returnvalue_9 (+ _returnvalue_2 2.0))
  (bind _returnvalue_10 (* _mainmeshinterval_4 _returnvalue_7))
  (bind _returnvalue_11 (* _mainmeshinterval_2 _returnvalue_9))
  (bind _returnvalue_12 (* _returnvalue_8 _mainmeshinterval_3))
  (bind _returnvalue_13 (* _returnvalue_6 _mainmeshinterval_5))
  (bind _returnvalue_14 (* _returnvalue_5 _mainmeshinterval))
  (bind _returnvalue_15 (Spline|GetTangentatDistanceAlongSpline _spline_5 _returnvalue_14 "Local"))
  (bind _returnvalue_16 (Spline|GetTangentatDistanceAlongSpline _spline_3 _returnvalue_13 "Local"))
  (bind (_refpoint _abspoint _impactnormal) (CallFunction|FindLandPoint _spline_4 _returnvalue_10 _needmatchland_2 0.0))
  (bind (_refpoint_2 _abspoint_2 _impactnormal_2) (CallFunction|FindLandPoint _spline_2 _returnvalue_12 _needmatchland_2 0.0))
  (bind (_refpoint_3 _abspoint_3 _impactnormal_3) (CallFunction|FindLandPoint _spline _returnvalue_11 _needmatchland 0.0))
  (Utilities|IsValid (Variables|Default|GetMainMesh)
    (:Is%20Valid
      (bind _output_get (LocalVariables|SetFenceCount (Math|Float|Ceil (/ (Spline|GetSplineLength (Variables|Default|GetSpline)) (Variables|Default|GetMainMeshInterval)))))
      (for _index (range 0 (- _output_get 1))
        (LocalVariables|SetTmpFenceIndex _index)
        (Utilities|FlowControl|Sequence
          (:then_0
            (LocalVariables|SetStartRefPoint _refpoint)
            (LocalVariables|SetStartWorldPoint _abspoint)
            (LocalVariables|SetStartNormal _impactnormal)
            (LocalVariables|SetEndRefPoint _refpoint_2)
            (LocalVariables|SetEndWorldPoint _abspoint_2)
            (LocalVariables|SetEndNormal _impactnormal_2)
            (LocalVariables|SetNextRefPoint _refpoint_3)
            (LocalVariables|SetNextWorldPoint _abspoint_3)
            (LocalVariables|SetNextNormal _impactnormal_3))
          (:then_1
            (bind _returnvalue_17 (AddComponent|AddSplineMeshComponent false))
            (bind _output_get_2 (LocalVariables|SetSplineMeshCom _returnvalue_17))
            (Components|StaticMesh|SetStaticMesh _output_get_2 (Variables|Default|GetMainMesh))
            (SplineMesh|SetStartandEnd (LocalVariables|GetSplineMeshCom) (+ (Math|Vector|SelectVector (- (LocalVariables|GetStartRefPoint) "0, 0,100.000000") (LocalVariables|GetStartRefPoint) (== (LocalVariables|GetTmpFenceIndex) 0)) _roadoffset) (Math|Vector|SelectVector (- _returnvalue_15 "0, 0,100.000000") _returnvalue_15 (== (LocalVariables|GetTmpFenceIndex) 0)) (+ (Math|Vector|SelectVector (- (LocalVariables|GetEndRefPoint) "0, 0,100.000000") (LocalVariables|GetEndRefPoint) (== (- (LocalVariables|GetFenceCount) 1) (LocalVariables|GetTmpFenceIndex))) _roadoffset) (Math|Vector|SelectVector (- _returnvalue_16 "0, 0,100.000000") _returnvalue_16 (== (- (LocalVariables|GetFenceCount) 1) (LocalVariables|GetTmpFenceIndex))) true :!class /Script/Engine.SplineMeshComponent)
            (Utilities|FlowControl|Sequence
              (:then_0
                (if (Variables|Default|GetmatchLandNormal)
                  (bind _outdeltaangle (CallFunction|GetRollingatPoint (- (LocalVariables|GetEndWorldPoint) (LocalVariables|GetStartWorldPoint)) (LocalVariables|GetStartNormal)))
                  (LocalVariables|SetSR (/ _outdeltaangle -57.324841))
                  (bind _outdeltaangle_2 (CallFunction|GetRollingatPoint (- (LocalVariables|GetEndWorldPoint) (LocalVariables|GetStartWorldPoint)) (/ (+ (LocalVariables|GetStartNormal) (LocalVariables|GetEndNormal) (LocalVariables|GetNextNormal)) 3.0)))
                  (LocalVariables|SetER (/ _outdeltaangle_2 -57.306591))
                  (Class|SplineMeshComponent|SetStartRoll (LocalVariables|GetSplineMeshCom) (Math|Float|SelectFloat (LocalVariables|GetSR) (LocalVariables|GetprevEndRoll) (== (LocalVariables|GetTmpFenceIndex) 0)) true)
                  (Class|SplineMeshComponent|SetEndRoll (LocalVariables|GetSplineMeshCom) (LocalVariables|GetER) true)
                  (LocalVariables|SetprevEndRoll (LocalVariables|GetER))))
              (:then_1
                (SplineMesh|SetStartScale (LocalVariables|GetSplineMeshCom) _returnvalue_3 true :!class /Script/Engine.SplineMeshComponent)
                (SplineMesh|SetEndScale (LocalVariables|GetSplineMeshCom) _returnvalue_3 true :!class /Script/Engine.SplineMeshComponent)
                (Collision|SetCollisionResponsetoChannel (LocalVariables|GetSplineMeshCom) "ECC_WorldStatic" "ECR_Block")
                (Collision|SetCollisionObjectType (LocalVariables|GetSplineMeshCom) "ECC_GameTraceChannel4")
                (Collision|SetCollisionResponsetoChannel (LocalVariables|GetSplineMeshCom) "ECC_PhysicsBody" "ECR_Block")
                (Collision|SetCollisionResponsetoChannel (LocalVariables|GetSplineMeshCom) "ECC_Pawn" "ECR_Block")
                (Collision|SetCollisionResponsetoChannel (LocalVariables|GetSplineMeshCom) "ECC_WorldStatic" "ECR_Block")
                (Collision|SetCollisionEnabled (LocalVariables|GetSplineMeshCom) "QueryAndPhysics")
                (Collision|SetCollisionResponsetoChannel (LocalVariables|GetSplineMeshCom) "ECC_Visibility" "ECR_Block")
                (Rendering|SetCastShadow (LocalVariables|GetSplineMeshCom) false)
                (Rendering|Material|SetMaterial (LocalVariables|GetSplineMeshCom) 0 (Variables|Default|GetRoadMaterial))
                (Collision|SetCollisionResponsetoChannel (LocalVariables|GetSplineMeshCom) "ECC_Camera" "ECR_Block"))
              (:then_2))))))))