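; Shared Blueprint utility library in the vehicle asset's Commons folder, providing angle, vector, distance and time math helpers.
; TrimAngle wraps angles to ±180 degrees and feeds the angle-to-vector and vector-to-rotator conversions, while DiffAngle finds the shortest signed difference.
; GetDeltaAngle combines these to return the pitch and yaw offsets from a source transform's facing toward a target.
; Standalone helpers cover signed 2D angle, pitch between points, actor distance and millisecond time-of-day timestamps.
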(fn AngleBetweenVector2D
  (params (targetVector :type Vector) (SelfVector :type Vector))
  (bind (_x _y) (Math|Vector|BreakVector SelfVector))
  (LocalVariables|SetDireCos (Class|KismetMathLibrary|VectorCosineAngle2D targetVector SelfVector))
  (LocalVariables|SetSV (Math|Vector|MakeVector _y (* -1 _x) 0.0))
  (if (> (Math|Vector|DotProduct (LocalVariables|GetSV) targetVector) 0.0)
    (LocalVariables|SetDeltaAngle (* (Class|KismetMathLibrary|DegAcos (LocalVariables|GetDireCos)) -1.0))
    (else
      (LocalVariables|SetDeltaAngle (Class|KismetMathLibrary|DegAcos (LocalVariables|GetDireCos)))))
  (return (LocalVariables|GetDeltaAngle)))

(fn DistBetweenActors
  (params (Actor1 :type Actor%20Object%20Reference) (Actor2 :type Actor%20Object%20Reference))
  (return (Math|Vector|VectorLength (- (Transformation|GetActorLocation Actor1) (Transformation|GetActorLocation Actor2)))))

(fn PitchAngleBetweenPoints
  (params (P1 :type Vector) (P2 :type Vector))
  (bind _returnvalue (- P1 P2))
  (return (Class|KismetMathLibrary|DegAsin (/ (.Z (Math|Vector|BreakVector _returnvalue)) (Math|Vector|VectorLength _returnvalue)))))

(fn Angle2Vector
  (params (Angle :type Float%20%28single-precision%29))
  (LocalVariables|SettmpVector (Math|Vector2D|Normalize2D (Math|Vector2D|MakeVector2D 1.0 (Math|Trig|Tan(Degrees) (CallFunction|TrimAngle Angle)))))
  (if (and (< Angle 9e+01) (> Angle -9e+01))
    (return (LocalVariables|GettmpVector))
    (else
      (return (* (LocalVariables|GettmpVector) -1.0)))))

(fn TrimAngle
  (params (Angle :type Float%20%28single-precision%29))
  (LocalVariables|SettmpAngle Angle)
  (LocalVariables|SetneedStop (not (and (<= (LocalVariables|GettmpAngle) 1.8e+02) (>= (LocalVariables|GettmpAngle) -1.8e+02))))
  (while (LocalVariables|GetneedStop)
    (if (> (LocalVariables|GettmpAngle) 1.8e+02)
      (LocalVariables|SettmpAngle (- (LocalVariables|GettmpAngle) 3.6e+02))
      (else
        (LocalVariables|SettmpAngle (+ (LocalVariables|GettmpAngle) 3.6e+02))))
    (LocalVariables|SetneedStop (not (and (<= (LocalVariables|GettmpAngle) 1.8e+02) (>= (LocalVariables|GettmpAngle) -1.8e+02)))))
  (return (LocalVariables|GettmpAngle)))

(fn DiffAngle
  (params (TargetAngle :type Float%20%28single-precision%29) (InputAngle :type Float%20%28single-precision%29))
  (bind _returnvalue (- TargetAngle InputAngle))
  (bind _returnvalue_2 (Math|Float|Absolute(Float) _returnvalue))
  (bind _returnvalue_3 (> _returnvalue_2 1.8e+02))
  (return (Math|Float|SelectFloat (* (* (Math|Float|Sign(Float) _returnvalue) (Math|Float|SelectFloat -1.0 1.0 _returnvalue_3)) (- 3.6e+02 _returnvalue_2)) _returnvalue _returnvalue_3)))

(fn VectorDirectionAngle
  (params (inVector :type Vector))
  (bind (_x _y) (Math|Vector|BreakVector inVector))
  (bind (_x_2 _y_2 _z) (Math|Vector|BreakVector inVector))
  (Utilities|FlowControl|Sequence
    (:then_0
      ;[1 1 1] 注释
      (LocalVariables|SetYaw (Class|KismetMathLibrary|DegAtan (/ _y_2 _x_2)))
      (LocalVariables|Setpitch (Class|KismetMathLibrary|DegAtan (/ _z (Math|Vector2D|Vector2DLength (Math|Vector2D|MakeVector2D _x_2 _y_2))))))
    (:then_1
      (LocalVariables|SetYaw (Math|Float|SelectFloat (LocalVariables|GetYaw) (Math|Float|SelectFloat (+ (LocalVariables|GetYaw) 1.8e+02) (+ (LocalVariables|GetYaw) -1.8e+02) (> _y 0.0)) (> _x 0.0))))
    (:then_2
      (return (Math|Rotator|MakeRotator 0.0 (CallFunction|TrimAngle (LocalVariables|Getpitch)) (CallFunction|TrimAngle (LocalVariables|GetYaw)))))))

(fn GetTimestamp
  (bind _returnvalue (Math|DateTime|Now))
  (bind (_year _month _day _hour _minute _second _millisecond) (Math|DateTime|BreakDateTime _returnvalue))
  (return (+ (* _hour 60000 60) (* _minute 1000 60) (* _second 1000) _millisecond)))

(fn GetDeltaAngle
  (params (SourceTrans :type Transform) (TargetTrans :type Transform))
  (bind _rotation (Math|Transform|BreakTransform SourceTrans))
  (bind _location (Math|Transform|BreakTransform SourceTrans))
  (bind _location_2 (Math|Transform|BreakTransform TargetTrans))
  (bind (_roll _pitch _yaw) (Math|Rotator|BreakRotator _rotation))
  (bind _returnvalue (- _location_2 _location))
  (bind _returnvalue_2 (CallFunction|VectorDirectionAngle _returnvalue))
  (LocalVariables|SetTarget%20Pitch (.pitch _returnvalue_2))
  (LocalVariables|SettargetYaw (.yaw _returnvalue_2))
  (LocalVariables|SetSourcePitch _pitch)
  (LocalVariables|SetSourceYaw _yaw)
  (return (CallFunction|DiffAngle (LocalVariables|GetTarget%20Pitch) (LocalVariables|GetSourcePitch)) (CallFunction|DiffAngle (LocalVariables|GettargetYaw) (LocalVariables|GetSourceYaw))))