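; Spline-placed fence that vehicles can knock over, built from instanced static meshes.
; The construction script spaces instances along the spline, optionally snapping them to the ground by line trace, with random location, rotation and scale noise.
; On overlap, HItAction marks nearby instances as fallen and pushes a hitting vehicle against its velocity according to its speed.
; Tick rolls those instances toward flat using delta-scaled steps.
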(event OnComponentBeginOverlap(FenceMeshComp)
  (params (OverlappedComponent :type Primitive%20Component%20Object%20Reference) (OtherActor :type Actor%20Object%20Reference) (OtherComp :type Primitive%20Component%20Object%20Reference) (OtherBodyIndex :type Integer) (bFromSweep :type Boolean) (SweepResult :type Hit%20Result%20Structure%20%28by%20ref%29))
  (bind (_outindex _returnvalue _needdown) (CallFunction|HItAction OtherActor SweepResult))
  (if _needdown
    (for _array_element _outindex
      (Utilities|Map|Add (Variables|Default|GetFallingMap) _array_element _returnvalue))))

(event EventBeginPlay)

(event Collision|EventActorBeginOverlap
  (params (OtherActor :type Actor%20Object%20Reference)))

(event EventTick
  (params (DeltaSeconds :type Float%20%28single-precision%29))
  (Variables|Default|SetD_Seconds DeltaSeconds)
  (if (> (Utilities|Map|Length (Variables|Default|GetFallingMap)) 0)
    (bind _keys (Utilities|Map|Keys (Variables|Default|GetFallingMap)))
    (for _array_element _keys
      (if (.ReturnValue (Utilities|Map|Find (Variables|Default|GetFallingMap) _array_element))
        (if (< (Math|Float|Absolute(Float) (+ (* (.Value (Utilities|Map|Find (Variables|Default|GetFallingMap) _array_element)) 7.0 (/ (Variables|Default|GetD_Seconds) 0.02)) (.Roll (Math|Rotator|BreakRotator (.rotation (.OutInstanceTransform (Components|InstancedStaticMesh|GetInstanceTransform (Variables|Default|GetFenceMeshComp) _array_element false))))))) 9e+01)
          (Components|InstancedStaticMesh|UpdateInstanceTransform (Variables|Default|GetFenceMeshComp) _array_element (Math|Transform|MakeTransform (.location (.OutInstanceTransform (Components|InstancedStaticMesh|GetInstanceTransform (Variables|Default|GetFenceMeshComp) _array_element false))) (Math|Rotator|MakeRotator (+ (* (.Value (Utilities|Map|Find (Variables|Default|GetFallingMap) _array_element)) 7.0 (/ (Variables|Default|GetD_Seconds) 0.02)) (.Roll (Math|Rotator|BreakRotator (.rotation (.OutInstanceTransform (Components|InstancedStaticMesh|GetInstanceTransform (Variables|Default|GetFenceMeshComp) _array_element false)))))) (.Pitch (Math|Rotator|BreakRotator (.rotation (.OutInstanceTransform (Components|InstancedStaticMesh|GetInstanceTransform (Variables|Default|GetFenceMeshComp) _array_element false))))) (.Yaw (Math|Rotator|BreakRotator (.rotation (.OutInstanceTransform (Components|InstancedStaticMesh|GetInstanceTransform (Variables|Default|GetFenceMeshComp) _array_element false)))))) (.scale (.OutInstanceTransform (Components|InstancedStaticMesh|GetInstanceTransform (Variables|Default|GetFenceMeshComp) _array_element false)))) false true false)
          (else
            (Utilities|Map|Remove (Variables|Default|GetFallingMap) _array_element)))))))

(fn ConstructionScript
  (bind _returnvalue (Math|Random|RandomUnitVector))
  (bind _returnvalue_2 (Math|Random|RandomUnitVector))
  (bind _returnvalue_3 (Math|Random|RandomUnitVector))
  (bind _returnvalue_4 (Math|Random|RandomUnitVector))
  (bind _rotnoise (Variables|Default|GetRotNoise))
  (bind _meshsize (Variables|Default|GetMeshSIze))
  (bind _needmatchland (Variables|Default|GetNeedMatchLand))
  (bind _locationnoise (Variables|Default|GetLocationNoise))
  (bind _rotation (Variables|Default|GetRotation))
  (bind (_x _y _z) (Math|Vector|BreakVector _meshsize))
  (bind _returnvalue_5 (- _returnvalue_2 _returnvalue))
  (bind _returnvalue_6 (- _returnvalue_3 _returnvalue_4))
  (bind _returnvalue_7 (* _rotation 1.0))
  (bind _returnvalue_8 (* _returnvalue_5 _rotnoise))
  (bind _returnvalue_9 (* _returnvalue_6 _locationnoise))
  (bind (_roll _pitch _yaw) (Math|Rotator|BreakRotator _returnvalue_7))
  (bind (_x_2 _y_2) (Math|Vector|BreakVector _returnvalue_9))
  (Utilities|FlowControl|Sequence
    (:then_0
      (Utilities|IsValid (Variables|Default|GetFenceMaterial)
        (:Is%20Valid
          (Rendering|Material|SetMaterial (Variables|Default|GetFenceMeshComp) 0 (Variables|Default|GetFenceMaterial)))))
    (:then_1
      (Components|StaticMesh|SetStaticMesh (Variables|Default|GetFenceMeshComp) (Variables|Default|GetFenceMesh))
      (bind _output_get (LocalVariables|SetFenceCount (Math|Float|Ceil (/ (Spline|GetSplineLength (Variables|Default|GetSpline)) (Variables|Default|GetFencePartLength)))))
      (for _index (range 1 (- _output_get 1))
        (bind _output_get_2 (LocalVariables|SettmpIndex _index))
        (LocalVariables|SetRefPoint (.RefPoint (CallFunction|FindLandPoint (Variables|Default|GetSpline) (* (Variables|Default|GetFencePartLength) (+ (Math|Conversions|ToFloat(Integer) _output_get_2) 0.0)) _needmatchland)))
        (LocalVariables|SetPartDirection (- (.ABSPoint (CallFunction|FindLandPoint (Variables|Default|GetSpline) (* (+ (Math|Conversions|ToFloat(Integer) _output_get_2) 1.0) (Variables|Default|GetFencePartLength)) _needmatchland)) (.ABSPoint (CallFunction|FindLandPoint (Variables|Default|GetSpline) (* (Variables|Default|GetFencePartLength) (+ (Math|Conversions|ToFloat(Integer) _output_get_2) 0.0)) _needmatchland))))
        (Utilities|FlowControl|Sequence
          (:then_0
            (Utilities|FlowControl|Sequence
              (:then_0
                (LocalVariables|SetBuildPoint (+ (LocalVariables|GetRefPoint) (Math|Vector|MakeVector _x_2 _y_2 0.0) (Variables|Default|GetMeshOffset))))
              (:then_1
                (LocalVariables|SetBuildRotate (Math|Rotator|MakeRotator (+ (.Roll (Math|Rotator|BreakRotator (Math|Rotator|MakeRotator (.Roll (Math|Rotator|BreakRotator (CallFunction|VectorDirectionAngle (LocalVariables|GetPartDirection)))) (.Pitch (Math|Rotator|BreakRotator (CallFunction|VectorDirectionAngle (LocalVariables|GetPartDirection)))) (select (Variables|Default|GetMatchSplineDir) (.Yaw (Math|Rotator|BreakRotator (CallFunction|VectorDirectionAngle (Spline|GetTangentatDistanceAlongSpline (Variables|Default|GetSpline) (* (LocalVariables|GettmpIndex) (Variables|Default|GetFencePartLength)) "Local")))) (.Yaw (Math|Rotator|BreakRotator (CallFunction|VectorDirectionAngle (LocalVariables|GetPartDirection)))))))) (.x _returnvalue_8) _roll) (+ (.Pitch (Math|Rotator|BreakRotator (Math|Rotator|MakeRotator (.Roll (Math|Rotator|BreakRotator (CallFunction|VectorDirectionAngle (LocalVariables|GetPartDirection)))) (.Pitch (Math|Rotator|BreakRotator (CallFunction|VectorDirectionAngle (LocalVariables|GetPartDirection)))) (select (Variables|Default|GetMatchSplineDir) (.Yaw (Math|Rotator|BreakRotator (CallFunction|VectorDirectionAngle (Spline|GetTangentatDistanceAlongSpline (Variables|Default|GetSpline) (* (LocalVariables|GettmpIndex) (Variables|Default|GetFencePartLength)) "Local")))) (.Yaw (Math|Rotator|BreakRotator (CallFunction|VectorDirectionAngle (LocalVariables|GetPartDirection)))))))) _pitch) (+ (.Yaw (Math|Rotator|BreakRotator (Math|Rotator|MakeRotator (.Roll (Math|Rotator|BreakRotator (CallFunction|VectorDirectionAngle (LocalVariables|GetPartDirection)))) (.Pitch (Math|Rotator|BreakRotator (CallFunction|VectorDirectionAngle (LocalVariables|GetPartDirection)))) (select (Variables|Default|GetMatchSplineDir) (.Yaw (Math|Rotator|BreakRotator (CallFunction|VectorDirectionAngle (Spline|GetTangentatDistanceAlongSpline (Variables|Default|GetSpline) (* (LocalVariables|GettmpIndex) (Variables|Default|GetFencePartLength)) "Local")))) (.Yaw (Math|Rotator|BreakRotator (CallFunction|VectorDirectionAngle (LocalVariables|GetPartDirection)))))))) (.z _returnvalue_8) _yaw))))
              (:then_2
                ;[1 1 1] 注释
                (LocalVariables|SetBuildSize (+ (Math|Vector|MakeVector (* (/ (Math|Vector|VectorLength (LocalVariables|GetPartDirection)) (Variables|Default|GetFencePartLength)) _x) _y _z) (* (- (Math|Random|RandomUnitVector) (Math|Random|RandomUnitVector)) (Variables|Default|GetSizeNoise)))))))
          (:then_1
            (Components|InstancedStaticMesh|AddInstance (Variables|Default|GetFenceMeshComp) (Math|Transform|MakeTransform (LocalVariables|GetBuildPoint) (LocalVariables|GetBuildRotate) (LocalVariables|GetBuildSize)))))))))

(fn FindLandPoint
  (params (inSpline :type Spline%20Component%20Object%20Reference) (positionInLine :type Float%20%28single-precision%29) (inNeedMatchLand :type Boolean))
  (bind _returnvalue (Spline|GetLocationatDistanceAlongSpline inSpline positionInLine "Local"))
  (bind _returnvalue_2 (Spline|GetLocationatDistanceAlongSpline inSpline positionInLine "Local"))
  (bind _returnvalue_3 (Spline|GetLocationatDistanceAlongSpline inSpline positionInLine "World"))
  (if inNeedMatchLand
    (bind (_outhit _returnvalue_4) (Collision|LineTraceForObjects (+ _returnvalue_3 "0, 0,10000.000000") (+ _returnvalue_3 "0, 0,-10000.000000") (LocalVariables|GetNewLocalVar_1) false 0 "None"))
    (if _returnvalue_4
      (bind _output_get (LocalVariables|SetLandLocation (.Location (Collision|BreakHitResult _outhit))))
      (return (Math|Transform|InverseTransformLocation (Transformation|GetWorldTransform inSpline) _output_get) _output_get)
      (else
        (return _returnvalue (Math|Transform|TransformLocation (Transformation|GetWorldTransform inSpline) _returnvalue))))
    (else
      (return _returnvalue_2 (Math|Transform|TransformLocation (Transformation|GetWorldTransform inSpline) _returnvalue_2)))))

(fn HItAction
  (params (inHitActor :type Actor%20Object%20Reference) (Sweep%20Result :type Hit%20Result%20Structure))
  (LocalVariables|SettmpHitActor inHitActor)
  (Utilities|FlowControl|Sequence
    (:then_0
      (for _index (range 0 (- (Components|InstancedStaticMesh|GetInstanceCount (Variables|Default|GetFenceMeshComp)) 1))
        (bind _output_get (LocalVariables|SetFenceIndex _index))
        (LocalVariables|SetHitDirection (- (+ (.Location (Math|Transform|BreakTransform (.OutInstanceTransform (Components|InstancedStaticMesh|GetInstanceTransform (Variables|Default|GetFenceMeshComp) _output_get true)))) (* (Math|Vector|GetForwardVector (.Rotation (Math|Transform|BreakTransform (.OutInstanceTransform (Components|InstancedStaticMesh|GetInstanceTransform (Variables|Default|GetFenceMeshComp) _output_get true))))) (/ (Variables|Default|GetCollisionLength) 2.0))) (Transformation|GetActorLocation (LocalVariables|GettmpHitActor))))
        (if (and (< (Math|Vector|VectorLengthXY (LocalVariables|GetHitDirection)) (/ 5e+02 1.0)) (not (Utilities|Set|Contains (Variables|Default|GetFallIndexSet) (LocalVariables|GetFenceIndex))))
          (LocalVariables|SetFallDir (Math|Float|SelectFloat 1.0 -1.0 (> (Math|Vector|DotProduct (Math|Vector|GetRightVector (.Rotation (Math|Transform|BreakTransform (.OutInstanceTransform (Components|InstancedStaticMesh|GetInstanceTransform (Variables|Default|GetFenceMeshComp) _output_get true))))) (LocalVariables|GetHitDirection)) 0.0)))
          (Utilities|Array|Add (LocalVariables|GetFallList) (LocalVariables|GetFenceIndex))
          (Utilities|Set|Add (Variables|Default|GetFallIndexSet) (LocalVariables|GetFenceIndex))))
      (bind _asbp_base_vehicle_pawn (Utilities|Casting|CastToBP_BaseVehiclePawn (LocalVariables|GettmpHitActor)))
      (bind _output_get_2 (Variables|Default|SetHIT%20VEHICLE _asbp_base_vehicle_pawn))
      (Physics|AddImpulse (Variables|/Game/VehicleAsset/BP_Vehicles/BP_BaseVehiclePawn.BP_BaseVehiclePawn_C|GetVehicleBody _output_get_2) (* (Math|Vector|Normalize (* (Transformation|GetComponentVelocity (Variables|/Game/VehicleAsset/BP_Vehicles/BP_BaseVehiclePawn.BP_BaseVehiclePawn_C|GetVehicleBody (Variables|Default|GetHIT%20VEHICLE))) -1.0)) (* (/ (Math|Float|Max(Float) (- (Default|GetSpeed (Variables|Default|GetHIT%20VEHICLE)) (Math|Float|Min(Float) (* (Variables|/Game/VehicleAsset/BP_Vehicles/BP_BaseVehiclePawn.BP_BaseVehiclePawn_C|GetMaxSpeed (Variables|Default|GetHIT%20VEHICLE)) 0.8) 5e+01)) 0.0) 2e+01) 2.5e+02)) "None" true))
    (:then_1
      (return (LocalVariables|GetFallList) (LocalVariables|GetFallDir) (> (Utilities|Array|Length (LocalVariables|GetFallList)) 0)))))