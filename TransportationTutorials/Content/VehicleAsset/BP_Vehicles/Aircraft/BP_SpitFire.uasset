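; BP_SpitFire is the Spitfire aircraft, a child Blueprint of a parent vehicle class.
; Its InitVehicle override calls the parent, then hands the Spitfire meshes to the Aileron, Wing, Rudder and Elevator objects, with separate left and right meshes for the ailerons.
; The event graph holds only disabled stubs and the construction script only calls its parent, so this class adds no other logic of its own.
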(event EventBeginPlay
  (|CallParentFunction) ; 此节点被禁用，将不会被调用。\n从引脚连出引线来编译功能。
)

(event Collision|EventActorBeginOverlap
  (params (OtherActor :type Actor%20Object%20Reference))
  (|CallParentFunction OtherActor) ; 此节点被禁用，将不会被调用。\n从引脚连出引线来编译功能。
)

(event EventTick
  (params (DeltaSeconds :type Float%20%28single-precision%29))
  (|CallParentFunction DeltaSeconds) ; 此节点被禁用，将不会被调用。\n从引脚连出引线来编译功能。
)

(fn ConstructionScript
  (|CallParentFunction))

(fn InitVehicle
  (|CallParentFunction)
  (Default|SetMeshComponent (Variables|Default|Getaileron) (Variables|Default|GetSpitfire_aileron_left) (Variables|Default|GetSpitfire_aileron_right))
  (Default|SetWingMeshComponent (Variables|Default|Getwing) (Variables|Default|GetSpitfire_wing))
  (Default|SetRudderMeshComponent (Variables|Default|Getrudder) (Variables|Default|GetSpitfire_rudder))
  (Default|SetElevatorMesh (Variables|Default|Getelevator) (Variables|Default|GetSpitfire_elevator)))