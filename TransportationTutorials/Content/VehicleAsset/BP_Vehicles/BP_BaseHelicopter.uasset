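; Base player-controlled helicopter built on the parent vehicle class, adding rotor flight to its wheeled landing-gear simulation.
; Construction sorts rotor components into main and tail; main rotors share lift scaled by power relative to hover, all spin with power.
; Input sets decaying roll/pitch targets, held by clamped proportional force-couple torques above a power threshold, while yaw is torqued directly.
; Tick runs control, flight, suspension, ruts and rotor-driven engine audio.
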(event EventTick
  (params (DeltaSeconds :type Float%20%28single-precision%29))
  ;[1 1 1] 车辆的实时状态模拟
  (Variables|Default|SetDeltaSeconds DeltaSeconds)
  (Utilities|FlowControl|Sequence
    (:then_1
      (Utilities|FlowControl|Sequence
        (:then_0
          ;;[1 1 1] 1. 载具控制信息更新
          (CallFunction|UpdateControlInfo))
        (:then_1
          ;;[1 1 1] 2. 飞行姿态与旋翼动作细节
          ;;;[1 1 1 1 12] 旋翼作用力控制
          (HelicopterPhysical|RotorForce)
          ;;;[1 1 1] 辅助维持飞机姿态
          (CallFunction|UpdateVehicleBodyState)
          ;;;[1 1 1] 架动作细节
          (CallFunction|UpdateVehicleMovement (Variables|Default|GetDeltaSeconds)))
        (:then_2
          ;;[1 1 1] 3. 起落架状态更新
          ;;;[1 1 1 1 12] 2. 载具环境输入：
          ;;; 处理地形起伏对车辆轮胎悬挂的影响
          (CallFunction|UpdateLandShapeInput)
          ;;;[1 1 1 1 12] 车轮/悬挂向车身施加支持力
          (CallFunction|UpdateSupportForce)
          ;;;[1 1 1 1 12] 施加车辆牵引力、阻力
          (CallFunction|UpdateTractionForce)
          ;;;[1 1 1 1 12] 施加车辆转向力
          (CallFunction|UpdateSteeringForce))
        (:then_3
          ;;[1 1 1] 4. 控制载具行驶效果
          ;;;[1 1 1] 印刷车辙
          (CallFunction|CreateRut)
          ;;;[1 1 1] 播放车辆音效
          (CallFunction|PlayVehicleSound))))))

(event Input|AxisEvents|InputAxisTurn
  (params (AxisValue :type Float%20%28single-precision%29))
  ;[1 1 1] 接受用户控制输入
  (CallFunction|LookARound AxisValue))

(event Input|AxisEvents|InputAxisLookUp
  (params (AxisValue :type Float%20%28single-precision%29))
  ;[1 1 1] 接受用户控制输入
  (CallFunction|LookUp AxisValue))

(event Input|AxisEvents|InputAxisMoveForward
  (params (AxisValue :type Float%20%28single-precision%29))
  ;[1 1 1] 接受用户控制输入
  (CallFunction|WheelForward AxisValue)
  (HelicopterControl|ControlHelicopterRot 0.0 AxisValue 0.0))

(event Input|AxisEvents|InputAxisBreak
  (params (AxisValue :type Float%20%28single-precision%29))
  ;[1 1 1] 接受用户控制输入
  (CallFunction|Break AxisValue))

(event Input|AxisEvents|InputAxisMoveRight
  (params (AxisValue :type Float%20%28single-precision%29))
  ;[1 1 1] 接受用户控制输入
  (CallFunction|WheelSteer AxisValue)
  (HelicopterControl|ControlHelicopterRot AxisValue 0.0 0.0))

(event Input|AxisEvents|InputAxisAircraftYawRight
  (params (AxisValue :type Float%20%28single-precision%29))
  ;[1 1 1] 接受用户控制输入
  (HelicopterControl|ControlHelicopterRot 0.0 0.0 AxisValue))

(event Input|AxisEvents|InputAxisRotorPowerUp
  (params (AxisValue :type Float%20%28single-precision%29))
  ;[1 1 1] 接受用户控制输入
  (HelicopterControl|MainRotorPowerUp AxisValue))

(fn ConstructionScript
  (|CallParentFunction)
  (bind _output_get (Variables|HelicopterStruct|SetRotorList (Actor|GetComponentsByClass "/Game/VehicleAsset/BP_Vehicles/Components/BP_CopterRotor.BP_CopterRotor_C")))
  (for _array_element _output_get
    (bind _output_get_2 (LocalVariables|SettmpRotor _array_element))
    (if (Variables|/Game/VehicleAsset/BP_Vehicles/Components/BP_CopterRotor.BP_CopterRotor_C|GetisMainRotor _output_get_2)
      (Utilities|Array|Add (Variables|Helicopterstruct|GetPowerTotorList) (LocalVariables|GettmpRotor))
      (else
        (Utilities|Array|Add (Variables|HelicopterStruct|GetTailTotor) (LocalVariables|GettmpRotor))))))

(fn MainRotorPowerUp
  (params (inDeltaPower :type Float%20%28single-precision%29))
  (LocalVariables|SetDP (* inDeltaPower 0.2))
  (if (> (Math|Float|Absolute(Float) (LocalVariables|GetDP)) 0.0)
    (Variables|HelicopterControl|SetRotorPower (Math|Float|Clamp(Float) (+ (Variables|HelicopterControl|GetRotorPower) (LocalVariables|GetDP)) 0.0 1e+02))
    (Variables|UpdateTimeRecord|SetRotorPowerUpdateTime 0.0)))

(fn ControlHelicopterRot
  (params (inRollValue :type Float%20%28single-precision%29) (inPitchValue :type Float%20%28single-precision%29) (inYawTurnValue :type Float%20%28single-precision%29))
  (bind _max_angle_degrees (Variables|Default|Getmax%20Angle%20Degrees))
  (bind _returnvalue (* _max_angle_degrees -1.0))
  (Utilities|FlowControl|Sequence
    (:then_0
      (LocalVariables|SetAPV (Math|Float|Absolute(Float) inPitchValue))
      (LocalVariables|SetARV (Math|Float|Absolute(Float) inRollValue))
      (LocalVariables|SetAYV (Math|Float|Absolute(Float) inYawTurnValue))
      (Variables|Default|SetPCV (+ (Variables|Default|GetPCV) inPitchValue)))
    (:then_1
      (if (> (+ (LocalVariables|GetAPV) (LocalVariables|GetARV) (LocalVariables|GetAYV)) 0.0)
        (Utilities|FlowControl|Sequence
          (:then_0
            (Variables|HelicopterControl|SetBodyRotTarget (Math|Rotator|MakeRotator (Math|Float|ClampAngle (+ (.Roll (Math|Rotator|BreakRotator (Variables|HelicopterControl|GetBodyRotTarget))) (* inRollValue 1.0)) _returnvalue _max_angle_degrees) (Math|Float|ClampAngle (+ (.Pitch (Math|Rotator|BreakRotator (Variables|HelicopterControl|GetBodyRotTarget))) (* inPitchValue -1.0 0.1)) _returnvalue _max_angle_degrees) (+ (.Yaw (Math|Rotator|BreakRotator (Variables|HelicopterControl|GetBodyRotTarget))) (* inYawTurnValue 1.0))))
            (Utilities|FlowControl|Sequence
              (:then_0
                (if (> (LocalVariables|GetARV) 0.0)
                  (Variables|UpdateTimeRecord|SetBodyRollUpdateTime 0.0)))
              (:then_1
                (if (> (LocalVariables|GetAPV) 0.0)
                  (Variables|UpdateTimeRecord|SetBodyPitchUpdateTime 0.0)))))
          (:then_1
            ;[1 1 1] 操控机身方向旋转
            (HelicopterPhysical|AddYawTorque inYawTurnValue 5e+06)))))))

(fn HelicopterMoveRight
  (params (moveRightValue :type Float%20%28single-precision%29)))

(fn RotorForce
  (for _array_element (Variables|Helicopterstruct|GetPowerTotorList)
    (Default|UpdateRotorForce _array_element (Variables|Default|GetVehicleBody) (* (/ (Variables|HelicopterControl|GetRotorPower) (Variables|Default|GethoverPercent)) (* (Variables|Default|GetvehicleMass) 9.8e+02 (/ 1.0 (Math|Conversions|ToFloat(Integer) (Utilities|Array|Length (Variables|Helicopterstruct|GetPowerTotorList)))))))))

(fn UpdateControlInfo
  (bind _hoverpercent (Variables|Default|GethoverPercent))
  (Utilities|FlowControl|Sequence
    (:then_0
      (|CallParentFunction))
    (:then_1
      ;[1 1 1] 更新主旋翼功率
      (bind _output_get (Variables|UpdateTimeRecord|SetRotorPowerUpdateTime (+ (Variables|UpdateTimeRecord|GetRotorPowerUpdateTime) (Variables|Default|GetDeltaSeconds))))
      (if (>= _output_get 0.2)
        (if (> (Variables|HelicopterControl|GetRotorPower) _hoverpercent)
          (Variables|HelicopterControl|SetRotorPower _hoverpercent)
          (else
            (Variables|HelicopterControl|SetRotorPower (Math|Float|Max(Float) (- (Variables|HelicopterControl|GetRotorPower) (* (Variables|Default|GetDeltaSeconds) (Math|Float|SelectFloat 3e+01 0.01 (Variables|Default|GetisWheelOnLand)))) 0.0))))))
    (:then_2
      (bind _output_get_2 (Variables|UpdateTimeRecord|SetBodyRollUpdateTime (+ (Variables|UpdateTimeRecord|GetBodyRollUpdateTime) (Variables|Default|GetDeltaSeconds))))
      (if (> _output_get_2 0.1)
        (Variables|HelicopterControl|SetBodyRotTarget (Math|Rotator|MakeRotator (* (.Roll (Math|Rotator|BreakRotator (Variables|HelicopterControl|GetBodyRotTarget))) 0.9) (.Pitch (Math|Rotator|BreakRotator (Variables|HelicopterControl|GetBodyRotTarget))) (.Yaw (Math|Rotator|BreakRotator (Variables|HelicopterControl|GetBodyRotTarget)))))))
    (:then_3
      (bind _output_get_3 (Variables|UpdateTimeRecord|SetBodyPitchUpdateTime (+ (Variables|UpdateTimeRecord|GetBodyPitchUpdateTime) (Variables|Default|GetDeltaSeconds))))
      (if (> _output_get_3 0.1)
        (Variables|HelicopterControl|SetBodyRotTarget (Math|Rotator|MakeRotator (.Roll (Math|Rotator|BreakRotator (Variables|HelicopterControl|GetBodyRotTarget))) (* (.Pitch (Math|Rotator|BreakRotator (Variables|HelicopterControl|GetBodyRotTarget))) (Math|Float|SelectFloat 0.9 0.998 (Variables|Default|GetisWheelOnLand))) (.Yaw (Math|Rotator|BreakRotator (Variables|HelicopterControl|GetBodyRotTarget)))))))))

(fn UpdateVehicleMovement
  (params (inDeltaSeconds :type Float%20%28single-precision%29))
  (|CallParentFunction inDeltaSeconds)
  (Utilities|FlowControl|Sequence
    (:then_0
      (for _array_element (Variables|Helicopterstruct|GetPowerTotorList)
        (Default|UpdateRotorRotation _array_element inDeltaSeconds (Variables|HelicopterControl|GetRotorPower) true)))
    (:then_1
      (for _array_element_2 (Variables|HelicopterStruct|GetTailTotor)
        (Default|UpdateRotorRotation _array_element_2 inDeltaSeconds (Variables|HelicopterControl|GetRotorPower) false)))))

(fn WheelForward
  (params (ThorttalControlValue :type Float%20%28single-precision%29))
  (LocalVariables|SetControlValue ThorttalControlValue)
  (|CallParentFunction (LocalVariables|GetControlValue)))

(fn UpdateCopterBodyRot
  (bind _vehiclebody (Variables|Default|GetVehicleBody))
  (bind _bodyrottarget (Variables|HelicopterControl|GetBodyRotTarget))
  (bind (_roll _pitch) (Math|Rotator|BreakRotator _bodyrottarget))
  (bind _returnvalue (Transformation|GetWorldRotation _vehiclebody))
  (bind (_roll_2 _pitch_2) (Math|Rotator|BreakRotator _returnvalue))
  ;[1 1 1] 旋翼功率达到门限时，启动辅助姿态控制
  (if (>= (Variables|HelicopterControl|GetRotorPower) 3e+01)
    (HelicopterPhysical|AddRollingTorque (Math|Float|Clamp(Float) (- _roll _roll_2) -1e+01 1e+01) 2e+05)
    (HelicopterPhysical|AddPitchTorque (Math|Float|Clamp(Float) (- _pitch _pitch_2) -1e+01 1e+01) 1e+06)))

(fn UpdateHUD
  (params (InputHUD :type Widget%20Speed%20UI%20Object%20Reference))
  (Utilities|IsValid InputHUD
    (:Is%20Valid
      (Rendering|Components|TextRender|SetText (Variables|/Game/VehicleAsset/widget/Widget_SpeedUI.Widget_SpeedUI_C|GetSpeedText InputHUD) (Utilities|Text|ToText(Float) (CallFunction|GetSpeed) "HalfToEven" false true 1 3 1 1))
      (Rendering|Components|TextRender|SetText (Variables|/Game/VehicleAsset/widget/Widget_SpeedUI.Widget_SpeedUI_C|GetThrottleValue InputHUD) (Utilities|Text|ToText(String) (Utilities|String|Append (Utilities|String|ToString(Text) (Utilities|Text|ToText(Float) (Variables|HelicopterControl|GetRotorPower) "HalfToEven" false true 1 3 0 0)) "%"))))))

(fn AddRollingTorque
  (params (InRollDirection :type Float%20%28single-precision%29) (Y :type Float%20%28single-precision%29))
  (Class|PrimitiveComponent|AddForceatLocationLocal (Variables|Default|GetVehicleBody) (* (Math|Vector|MakeVector 0.0 Y 0.0) InRollDirection) "0.000000, 0,500.000000" "None")
  (Class|PrimitiveComponent|AddForceatLocationLocal (Variables|Default|GetVehicleBody) (* (Math|Vector|MakeVector 0.0 Y 0.0) (* InRollDirection -1.0)) "0.000000, 0,-500.000000" "None"))

(fn AddPitchTorque
  (params (PitchDirection :type Float%20%28single-precision%29) (Z :type Float%20%28single-precision%29))
  (Class|PrimitiveComponent|AddForceatLocationLocal (Variables|Default|GetVehicleBody) (* (Math|Vector|MakeVector 0.0 0.0 Z) PitchDirection) "500.000000, 0, 0" "None")
  (Class|PrimitiveComponent|AddForceatLocationLocal (Variables|Default|GetVehicleBody) (* (Math|Vector|MakeVector 0.0 0.0 Z) (* PitchDirection -1.0)) "-500.000000, 0, 0" "None"))

(fn AddYawTorque
  (params (YDirection :type Float%20%28single-precision%29) (Y :type Float%20%28single-precision%29))
  (Class|PrimitiveComponent|AddForceatLocationLocal (Variables|Default|GetVehicleBody) (* (Math|Vector|MakeVector 0.0 Y 0.0) YDirection) "500.000000, 0, 0" "None")
  (Class|PrimitiveComponent|AddForceatLocationLocal (Variables|Default|GetVehicleBody) (* (Math|Vector|MakeVector 0.0 Y 0.0) (* YDirection -1.0)) "-500.000000, 0, 0" "None"))

(fn UpdateVehicleBodyState
  (|CallParentFunction)
  (TickUpdateMovement|UpdateCopterBodyRot))

(fn PlayVehicleSound
  (bind _rotorpower (Variables|HelicopterControl|GetRotorPower))
  (bind _returnvalue (/ _rotorpower 1e+02))
  (if (Class|Pawn|IsControlled)
    (Utilities|FlowControl|Sequence
      (:then_0
        ;[1 1 1] 车辆引擎音效
        (if (not (Audio|Components|Audio|IsPlaying (Variables|Default|GetEngineLoopSound)))
          ;;[1 1 1] 注释
          (Variables|/Script/Engine.AudioComponent|SetSound (Variables|Default|GetEngineLoopSound) (Variables|Default|GetRunningLoopSound))
          (Audio|Components|Audio|Play (Variables|Default|GetEngineLoopSound) 0.0)
          (else
            ;;[1 1 1] 根据车辆状态调整音效
            (Audio|Parameter|SetFloatParameter (Variables|Default|GetEngineLoopSound) "RPM" _returnvalue :!class /Script/Engine.AudioComponent)
            (Audio|Parameter|SetFloatParameter (Variables|Default|GetEngineLoopSound) "THR" _returnvalue :!class /Script/Engine.AudioComponent)
            (if (> (Utilities|Array|Length (Variables|Helicopterstruct|GetPowerTotorList)) 0)
              (Audio|Parameter|SetFloatParameter (Variables|Default|GetEngineLoopSound) "RotorRPM" (/ (Variables|/Game/VehicleAsset/BP_Vehicles/Components/BP_CopterRotor.BP_CopterRotor_C|GetRotSpeed (Utilities|Array|Get(acopy) (Variables|Helicopterstruct|GetPowerTotorList))) 7e+02) :!class /Script/Engine.AudioComponent)))))
      (:then_1
        ;[1 1 1] 刹车音效
        (bind _output_get (LocalVariables|SetBRK (* (Math|Float|Clamp(Float) (* (- (/ (Variables|Default|GetBreakForce) (Variables|Default|GetMaxBreakForce)) 0.1) 1.111111)) (Math|Float|Clamp(Float) (/ (- (CallFunction|GetSpeed) 4e+01) 5e+01)))))
        (if (> _output_get 0.01)
          (if (Variables|Default|GetisWheelOnLand)
            (CallFunction|BreakSoundEvent)
            (Audio|Parameter|SetFloatParameter (Variables|Default|GetBreakSoundPlayer) "BRK" (LocalVariables|GetBRK) :!class /Script/Engine.AudioComponent)))))))