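; Base fixed-wing aircraft pawn that extends a parent vehicle Blueprint with flight control surfaces.
; InitVehicle adds aileron, wing, rudder and elevator components after the parent setup.
; Movement axes drive both wheels and surfaces, with opposed aileron deltas for roll, while RotorPowerUp is an empty stub.
; Tick runs the ground-vehicle pipeline: control and terrain input, support, traction and steering forces, body state, ruts and sound.
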(event EventBeginPlay
  (|CallParentFunction) ; 此节点被禁用，将不会被调用。\n从引脚连出引线来编译功能。
)

(event Collision|EventActorBeginOverlap
  (params (OtherActor :type Actor%20Object%20Reference)))

(event EventTick
  (params (DeltaSeconds :type Float%20%28single-precision%29))
  ;[1 1 1] 车辆的实时状态模拟
  (Variables|Default|SetDeltaSeconds DeltaSeconds)
  (Utilities|FlowControl|Sequence
    (:then_1
      (Utilities|FlowControl|Sequence
        (:then_0
          ;;[1 1 1] 1. 车辆控制信息更新
          (CallFunction|UpdateControlInfo)
          ;;[1 1 1] 2. 车辆环境输入：
          ;; 处理地形起伏对车辆轮胎悬挂的影响
          (CallFunction|UpdateLandShapeInput))
        (:then_1
          ;;[1 1 1] 3. 车身物理状态更新
          ;;;[1 1 1 1 12] 车轮/悬挂向车身施加支持力
          (CallFunction|UpdateSupportForce)
          ;;;[1 1 1 1 12] 施加车辆牵引力、阻力
          (CallFunction|UpdateTractionForce)
          ;;;[1 1 1 1 12] 施加车辆转向力
          (CallFunction|UpdateSteeringForce))
        (:then_2
          ;;[1 1 1] 4. 车辆动作细节
          (CallFunction|UpdateVehicleMovement (Variables|Default|GetDeltaSeconds))
          ;;[1 1 1] 管控车身姿态，处置翻车
          (CallFunction|UpdateVehicleBodyState))
        (:then_3
          ;;[1 1 1] 5. 控制车辆行驶效果
          ;;;[1 1 1] 印刷车辙
          (CallFunction|CreateRut)
          ;;;[1 1 1] 播放车辆音效
          (CallFunction|PlayVehicleSound))))))

(event Input|AxisEvents|InputAxisTurn
  (params (AxisValue :type Float%20%28single-precision%29))
  ;[1 1 1] 接受用户控制输入
  ;;[1 1 1] 视角操控
  (CallFunction|LookARound AxisValue))

(event Input|AxisEvents|InputAxisLookUp
  (params (AxisValue :type Float%20%28single-precision%29))
  ;[1 1 1] 接受用户控制输入
  ;;[1 1 1] 视角操控
  (CallFunction|LookUp AxisValue))

(event Input|AxisEvents|InputAxisMoveForward
  (params (AxisValue :type Float%20%28single-precision%29))
  ;[1 1 1] 接受用户控制输入
  (if (> (Math|Float|Absolute(Float) AxisValue) 0.0)
    (CallFunction|WheelForward AxisValue)
    (AircraftOperation|PlanePitchOperation AxisValue)))

(event Input|AxisEvents|InputAxisBreak
  (params (AxisValue :type Float%20%28single-precision%29))
  ;[1 1 1] 接受用户控制输入
  (CallFunction|Break AxisValue))

(event Input|AxisEvents|InputAxisMoveRight
  (params (AxisValue :type Float%20%28single-precision%29))
  ;[1 1 1] 接受用户控制输入
  (if (> (Math|Float|Absolute(Float) AxisValue) 0.0)
    (CallFunction|WheelSteer AxisValue)
    (AircraftOperation|PlaneRollOperation AxisValue)))

(event Input|AxisEvents|InputAxisRotorPowerUp
  (params (AxisValue :type Float%20%28single-precision%29))
  ;[1 1 1] 接受用户控制输入
  (if (> (Math|Float|Absolute(Float) AxisValue) 0.0)
    (AircraftOperation|RotorPowerUp AxisValue)))

(event Input|AxisEvents|InputAxisAircraftYawRight
  (params (AxisValue :type Float%20%28single-precision%29))
  ;[1 1 1] 接受用户控制输入
  (if (> (Math|Float|Absolute(Float) AxisValue) 0.0)
    (AircraftOperation|PlaneYawOperation AxisValue)))

(fn ConstructionScript
  (|CallParentFunction))

(fn RotorPowerUp
  (params (d_RotorPower :type Float%20%28single-precision%29)))

(fn WheelForward
  (params (ThorttalControlValue :type Float%20%28single-precision%29))
  (|CallParentFunction ThorttalControlValue))

(fn PlanePitchOperation
  (params (dValue :type Float%20%28single-precision%29))
  (Default|UpdateElevatorAngle (Variables|AircraftComponent|Getelevator) dValue))

(fn PlaneRollOperation
  (params (DValue :type Float%20%28single-precision%29))
  (LocalVariables|Setdelta%20value DValue)
  (Default|UpdateAileronAngle (Variables|AircraftComponent|Getaileron) (LocalVariables|Getdelta%20value) (* (LocalVariables|Getdelta%20value) -1.0)))

(fn PlaneYawOperation
  (params (DValue :type Float%20%28single-precision%29))
  (Default|UpdateRudderAngle (Variables|AircraftComponent|Getrudder) DValue))

(fn 新函数0)

(fn InitVehicle
  (|CallParentFunction)
  ;[1 1 1] 初始化飞行组件
  (Utilities|FlowControl|Sequence
    (:then_0
      (bind _returnvalue (Game|AddComponentbyClass "/Game/VehicleAsset/BP_Vehicles/Aircraft/BP_AileronComponent.BP_AileronComponent_C"))
      (Variables|AircraftComponent|Setaileron _returnvalue))
    (:then_1
      (bind _returnvalue_2 (Game|AddComponentbyClass "/Game/VehicleAsset/BP_Vehicles/Aircraft/BP_AircraftWing.BP_AircraftWing_C"))
      (Variables|AircraftComponent|Setwing _returnvalue_2))
    (:then_2
      (bind _returnvalue_3 (Game|AddComponentbyClass "/Game/VehicleAsset/BP_Vehicles/Aircraft/BP_AircraftRudder.BP_AircraftRudder_C"))
      (Variables|AircraftComponent|Setrudder _returnvalue_3))
    (:then_3
      (bind _returnvalue_4 (Game|AddComponentbyClass "/Game/VehicleAsset/BP_Vehicles/Aircraft/BP_AircraftElevator.BP_AircraftElevator_C"))
      (Variables|AircraftComponent|Setelevator _returnvalue_4))))