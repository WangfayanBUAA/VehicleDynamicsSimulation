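; T-72 tracked vehicle Blueprint that specializes a parent vehicle class with this tank's wheel layout.
; RegistTrackWheel fills the LeftWheels and RightWheels arrays with eight BPVehicleWheel components per side.
; The construction script only calls the parent, and the event graph holds only disabled stubs, so the file adds no other logic of its own.
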(event EventBeginPlay
  (|CallParentFunction) ; 此节点被禁用，将不会被调用。\n从引脚连出引线来编译功能。
)

(event Collision|EventActorBeginOverlap
  (params (OtherActor :type Actor%20Object%20Reference))
  (|CallParentFunction OtherActor) ; 此节点被禁用，将不会被调用。\n从引脚连出引线来编译功能。
)

(event EventTick
  (params (DeltaSeconds :type Float%20%28single-precision%29))
  (|CallParentFunction DeltaSeconds) ; 此节点被禁用，将不会被调用。\n从引脚连出引线来编译功能。
)

(fn ConstructionScript
  (|CallParentFunction))

(fn RegistTrackWheel
  (Variables|Default|SetLeftWheels (Utilities|Array|MakeArray (Variables|Default|GetBP_VehicleWheel9) (Variables|Default|GetBP_VehicleWheel10) (Variables|Default|GetBP_VehicleWheel11) (Variables|Default|GetBP_VehicleWheel12) (Variables|Default|GetBP_VehicleWheel13) (Variables|Default|GetBP_VehicleWheel14) (Variables|Default|GetBP_VehicleWheel16) (Variables|Default|GetBP_VehicleWheel17)))
  (Variables|Default|SetRightWheels (Utilities|Array|MakeArray (Variables|Default|GetBP_VehicleWheel) (Variables|Default|GetBP_VehicleWheel1) (Variables|Default|GetBP_VehicleWheel2) (Variables|Default|GetBP_VehicleWheel3) (Variables|Default|GetBP_VehicleWheel4) (Variables|Default|GetBP_VehicleWheel5) (Variables|Default|GetBP_VehicleWheel7) (Variables|Default|GetBP_VehicleWheel8))))