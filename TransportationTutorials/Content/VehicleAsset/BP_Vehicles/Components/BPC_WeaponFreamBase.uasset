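; Vehicle weapon mount component that yaws itself and pitches its Weapon, either from turn input or toward a locked world direction.
; Input, which accelerates while held, feeds pending TargetYaw and TargetPitch deltas through AddFreamPosition, or shifts LockTargetRotator while locked.
; Each Tick consumes those deltas at capped speeds, then MoveToLockTarget re-queues the error to the lock direction, stabilizing aim.
; Helpers set absolute angles, toggle locking, zero or stop movement.
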(event EventBeginPlay)

(event EventTick
  (params (DeltaSeconds :type Float%20%28single-precision%29))
  (Variables|WeaponMoveMent|SetdeltaSeconds DeltaSeconds)
  (WeaponMovement|UpdateFreamYaw)
  (WeaponMovement|UpdateFreamPitch)
  (WeaponControl|MovetoLockTarget))

(fn AddFreamPosition
  (params (input_yaw :type Float%20%28single-precision%29) (input_pitch :type Float%20%28single-precision%29))
  (bind _weapon (Variables|Default|Getweapon))
  (bind _returnvalue (Transformation|GetRelativeTransform _weapon))
  (Utilities|FlowControl|Sequence
    (:then_0
      (if (<= (Math|Float|Absolute(Float) (Variables|WeaponMoveMent|GettargetYaw)) (Variables|WeaponMoveMent|GetmaxTargetYawDiff))
        (if (or (Math|Boolean|ANDBoolean (<= (+ input_yaw (Variables|WeaponMoveMent|GettargetYaw)) 9e+01) (>= (+ input_yaw (Variables|WeaponMoveMent|GettargetYaw)) -9e+01) (<= (Math|Float|Absolute(Float) (- (Variables|WeaponMoveMent|GettargetYaw) (.Yaw (Math|Rotator|BreakRotator (.rotation (Transformation|GetRelativeTransform)))))) 1.0)) (not (Variables|WeaponMoveMent|GetNeedMaxYaw)))
          (bind _output_get (Variables|WeaponMoveMent|SettargetYaw (+ input_yaw (Variables|WeaponMoveMent|GettargetYaw))))
          (Development|PrintString (Utilities|String|ToString(Float) _output_get))
          (else
            (Development|PrintString "Hello")))))
    (:then_1
      (if (< (Math|Float|Absolute(Float) (Variables|WeaponMoveMent|GettargetPitch)) 5.0)
        (Variables|WeaponMoveMent|SettargetPitch (Math|Float|Clamp(Float) (+ input_pitch (Variables|WeaponMoveMent|GettargetPitch)) (- (Variables|WeaponMoveMent|GetMinPitch) (.pitch (.rotation _returnvalue))) (- (Variables|WeaponMoveMent|GetMaxPitch) (.pitch (.rotation _returnvalue)))))))))

(fn UpdateFreamYaw
  (bind _maxspeed_yaw (Variables|WeaponMoveMent|GetmaxSpeed_Yaw))
  (bind _returnvalue (* 2 _maxspeed_yaw))
  (Variables|WeaponMoveMent|SetSpeedYaw (Math|Float|SelectFloat (Math|Float|Min(Float) (+ (Variables|WeaponMoveMent|GetSpeedYaw) 0.5) _returnvalue) (Math|Float|Min(Float) (+ (Variables|WeaponMoveMent|GetSpeedYaw) 1.0) _returnvalue) (Variables|WeaponControl|GetWeaponLockDirection)))
  (LocalVariables|Setposition (.rotation (Transformation|GetRelativeTransform)))
  (bind _output_get (LocalVariables|SetTurnAngle (* (Math|Float|Sign(Float) (Variables|WeaponMoveMent|GettargetYaw)) (Math|Float|Min(Float) (Math|Float|Absolute(Float) (Variables|WeaponMoveMent|GettargetYaw)) (* (Variables|WeaponMoveMent|GetSpeedYaw) (Variables|WeaponMoveMent|GetdeltaSeconds))))))
  (Transformation|SetRelativeRotation (Math|Rotator|MakeRotator (.roll (LocalVariables|Getposition)) (.pitch (LocalVariables|Getposition)) (+ (.yaw (LocalVariables|Getposition)) _output_get)) false false)
  (Variables|WeaponMoveMent|SettargetYaw (- (Variables|WeaponMoveMent|GettargetYaw) (LocalVariables|GetTurnAngle))))

(fn UpdateFreamPitch
  (bind _maxspeed_pitch (Variables|Default|GetMaxSpeed_Pitch))
  (bind _deltaseconds (Variables|WeaponMoveMent|GetdeltaSeconds))
  (bind _returnvalue (* _maxspeed_pitch _deltaseconds))
  (bind _output_get (LocalVariables|SetsocketPos (.rotation (Transformation|GetRelativeTransform (Variables|Default|Getweapon)))))
  (LocalVariables|SetcurrentPitch (.pitch _output_get))
  (bind _output_get_2 (LocalVariables|SetmovePitch (* (Math|Float|Sign(Float) (Variables|WeaponMoveMent|GettargetPitch)) (Math|Float|Min(Float) (Math|Float|Absolute(Float) (Variables|WeaponMoveMent|GettargetPitch)) (Math|Float|SelectFloat (* _returnvalue 0.1) _returnvalue (Variables|Default|GetSlow%20Lock))))))
  (Transformation|SetRelativeRotation (Variables|Default|Getweapon) (Math|Rotator|MakeRotator (.roll (LocalVariables|GetsocketPos)) (+ (.pitch (LocalVariables|GetsocketPos)) _output_get_2) (.yaw (LocalVariables|GetsocketPos))) false false)
  (Variables|WeaponMoveMent|SettargetPitch (- (Variables|WeaponMoveMent|GettargetPitch) (LocalVariables|GetmovePitch))))

(fn SetFreamPosition
  (params (input_yaw :type Float%20%28single-precision%29) (input_pitch :type Float%20%28single-precision%29) (setYaw :type Boolean) (setPitch :type Boolean))
  (LocalVariables|SetFreamRotation (.rotation (Transformation|GetRelativeTransform)))
  (LocalVariables|SetWeaponRotation (.rotation (Transformation|GetRelativeTransform (Variables|Default|Getweapon))))
  (Utilities|FlowControl|Sequence
    (:then_0
      (if (Math|Boolean|ANDBoolean (<= input_yaw 1.8e+02) (>= input_yaw -1.8e+02) setYaw)
        (Variables|WeaponMoveMent|SettargetYaw (- input_yaw (.yaw (LocalVariables|GetFreamRotation))))))
    (:then_1
      (if (Math|Boolean|ANDBoolean (<= input_pitch 1.8e+02) (>= input_pitch -1.8e+02) setPitch)
        (Variables|WeaponMoveMent|SettargetPitch (- input_pitch (.pitch (LocalVariables|GetWeaponRotation))))))))

(fn GetPosition
  (return (.Yaw (Math|Rotator|BreakRotator (.rotation (Transformation|GetRelativeTransform)))) (.Pitch (Math|Rotator|BreakRotator (.rotation (Transformation|GetRelativeTransform (Variables|Default|Getweapon)))))))

(fn DebugShowDirection
  (params (Start :type Vector) (Direction :type Vector) (Length :type Float%20%28single-precision%29) (LineColor :type Linear%20Color%20Structure) (Duration :type Float%20%28single-precision%29) (Radius :type Float%20%28single-precision%29))
  (Class|KismetSystemLibrary|DrawDebugCylinder Start (+ Start (* Direction Length)) Radius 12 LineColor Duration 1.0))

(fn TurnRight
  (params (AxisValue :type Float%20%28single-precision%29))
  (bind _weapon (Variables|Default|Getweapon))
  (bind _maxtargetyawdiff (Variables|WeaponMoveMent|GetmaxTargetYawDiff))
  (bind _returnvalue (Transformation|GetWorldRotation _weapon))
  (bind _yaw (Math|Rotator|BreakRotator _returnvalue))
  (if (> (Math|Float|Absolute(Float) AxisValue) 0.0)
    (if (Variables|WeaponControl|GetWeaponLockDirection)
      (Variables|WeaponControl|SetInputYawIncreaceStep (+ (Variables|WeaponControl|GetInputYawIncreaceStep) 0.005))
      (LocalVariables|SetnextYaw (select (< (Math|Float|Absolute(Float) (CallFunction|DiffAngle (CallFunction|TrimAngle (+ (.yaw (Variables|WeaponControl|GetLockTargetRotator)) (* (Variables|WeaponControl|GetInputYawIncreaceStep) (Math|Float|Sign(Float) AxisValue)))) _yaw)) _maxtargetyawdiff) (CallFunction|TrimAngle (+ (.yaw (Variables|WeaponControl|GetLockTargetRotator)) (* (Variables|WeaponControl|GetInputYawIncreaceStep) (Math|Float|Sign(Float) AxisValue)))) (CallFunction|TrimAngle (+ _yaw (* (Math|Float|Sign(Float) (CallFunction|DiffAngle (CallFunction|TrimAngle (+ (.yaw (Variables|WeaponControl|GetLockTargetRotator)) (* (Variables|WeaponControl|GetInputYawIncreaceStep) (Math|Float|Sign(Float) AxisValue)))) _yaw)) _maxtargetyawdiff)))))
      (Variables|WeaponControl|SetLockTargetRotator (Math|Rotator|MakeRotator (.roll (Variables|WeaponControl|GetLockTargetRotator)) (.pitch (Variables|WeaponControl|GetLockTargetRotator)) (LocalVariables|GetnextYaw)))
      (else
        (Variables|WeaponControl|SetInputYawIncreaceStep (+ (Variables|WeaponControl|GetInputYawIncreaceStep) 0.1))
        (InputInterface|AddFreamPosition (* (Variables|WeaponControl|GetInputYawIncreaceStep) (Math|Float|Sign(Float) AxisValue)) 0.0)))
    (else
      (Variables|WeaponControl|SetInputYawIncreaceStep 0.0))))

(fn TurnUp
  (params (AxisValue :type Float%20%28single-precision%29))
  (if (> (Math|Float|Absolute(Float) AxisValue) 0.0)
    (if (Variables|WeaponControl|GetWeaponLockDirection)
      (Variables|WeaponControl|SetInputPitchIncreaceStep (+ (Variables|WeaponControl|GetInputPitchIncreaceStep) 0.001))
      (Variables|WeaponControl|SetLockTargetRotator (Math|Rotator|MakeRotator (.roll (Variables|WeaponControl|GetLockTargetRotator)) (Math|Float|Clamp(Float) (+ (.pitch (Variables|WeaponControl|GetLockTargetRotator)) (* (Variables|WeaponControl|GetInputPitchIncreaceStep) (Math|Float|Sign(Float) AxisValue))) (Variables|WeaponMoveMent|GetMinPitch) (Variables|WeaponMoveMent|GetMaxPitch)) (.yaw (Variables|WeaponControl|GetLockTargetRotator))))
      (else
        (Variables|WeaponControl|SetInputPitchIncreaceStep (+ (Variables|WeaponControl|GetInputPitchIncreaceStep) 0.02))
        (InputInterface|AddFreamPosition 0.0 (* (Variables|WeaponControl|GetInputPitchIncreaceStep) (Math|Float|Sign(Float) AxisValue)))))
    (else
      (Variables|WeaponControl|SetInputPitchIncreaceStep 0.0))))

(fn LockWeaponDirection
  (params (needLock :type Boolean) (SLowLock :type Boolean) (InputLockTarget :type Rotator))
  (Variables|Default|SetSlow%20Lock SLowLock)
  (bind _output_get (Variables|WeaponControl|SetWeaponLockDirection needLock))
  (if _output_get
    (Variables|WeaponControl|SetLockTargetRotator InputLockTarget)))

(fn MovetoLockTarget
  (bind _locktargetrotator (Variables|WeaponControl|GetLockTargetRotator))
  (bind _weapon (Variables|Default|Getweapon))
  (bind _returnvalue (Transformation|GetWorldRotation _weapon))
  (bind _returnvalue_2 (CallFunction|DiffAngle (.yaw _locktargetrotator) (.yaw _returnvalue)))
  (if (Variables|WeaponControl|GetWeaponLockDirection)
    (InputInterface|AddFreamPosition self _returnvalue_2 (Math|Float|Clamp(Float) (- (.pitch _locktargetrotator) (.pitch _returnvalue)) -1.0))
    (if (< (* (Variables|WeaponMoveMent|GettargetYaw) _returnvalue_2) 0.0)
      (Variables|WeaponMoveMent|SettargetYaw 0.0))))

(fn ZeroWeapon
  (InputInterface|LockWeaponDirection false false "0, 0, 0")
  (WeaponMovement|SetFreamPosition 0.0 0.0 true true))

(fn FireLockWeaponPosition
  (params (ISLock :type Boolean))
  (Variables|WeaponControl|SetWeaponLockDirection (not ISLock)))

(fn StopMove
  (Variables|WeaponMoveMent|SettargetYaw 0.0)
  (Variables|WeaponMoveMent|SettargetPitch 0.0))