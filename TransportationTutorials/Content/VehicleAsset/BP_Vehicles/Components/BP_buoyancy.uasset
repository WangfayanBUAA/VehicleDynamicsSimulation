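; BP_buoyancy is a vehicle component that computes buoyancy at its location, treating the water surface like a suspension spring.
; InitBuoyancy stores the water surface, and UpdateSuspensionLength measures the component's height above the water, capped at the natural suspension length.
; GetPressure turns that length and its rate of change into a clamped spring-damper force.
; GetSupportVector returns the forces with the component's up vector, leaving their application to the caller.
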(event EventBeginPlay
  (|CallParentFunction) ; This node is disabled and will not be called.\nDrag off pins to build functionality.
)

(event EventTick
  (params (DeltaSeconds :type Float%20%28single-precision%29))
  (|CallParentFunction DeltaSeconds) ; This node is disabled and will not be called.\nDrag off pins to build functionality.
)

(event EventTick
  (params (DeltaSeconds :type Float%20%28single-precision%29)))

(fn GetSupportVector
  (params (DeltaSeconds :type Float%20%28single-precision%29))
  (bind (_pressure _springforce _dampforce) (CallFunction|GetPressure DeltaSeconds))
  (return _pressure _springforce _dampforce (Math|Vector|GetUpVector (.Rotation (Math|Transform|BreakTransform (Transformation|GetWorldTransform self))))))

(fn UpdateSuspensionLength
  (params (DeltaSeconds :type Float%20%28single-precision%29))
  (Variables|Default|SetLastSuspLength (Variables|Default|GetSuspLength))
  (bind _output_get (LocalVariables|SetsuspLocation (Transformation|GetWorldLocation self)))
  (bind _output_get_2 (Variables|Default|SetSuspLength (Math|Float|Min(Float) (- (.Z (Math|Vector|BreakVector _output_get)) (Default|GetWaterHeightatLocation (Variables|Default|GetwaterSurface) (Math|Vector2D|MakeVector2D (.X (Math|Vector|BreakVector _output_get)) (.Y (Math|Vector|BreakVector _output_get))))) (Variables|Default|GetNatureSuspensionLength))))
  (return))

(fn InitBuoyancy
  (params (waterSurface :type BP%20Water%20Surface%20Object%20Reference))
  (Variables|Default|SetwaterSurface waterSurface))

(fn GetPressure
  (params (DeltaSeconds :type Float%20%28single-precision%29))
  (LocalVariables|SetDS DeltaSeconds)
  (LocalVariables|SetTempMaxForce (* (Variables|Default|GetNatureSuspensionLength) (Variables|Default|GetSuspStrength) 1.5))
  (return (Math|Float|Clamp(Float) (+ (Math|Float|Clamp(Float) (* (- (Variables|Default|GetNatureSuspensionLength) (Variables|Default|GetSuspLength)) (Variables|Default|GetSuspStrength)) 0.0 (LocalVariables|GetTempMaxForce)) (* (/ (- (Variables|Default|GetSuspLength) (Variables|Default|GetLastSuspLength)) (LocalVariables|GetDS)) (Variables|Default|GetSuspensonDamp) -1.0)) (* (LocalVariables|GetTempMaxForce) -1.0) (LocalVariables|GetTempMaxForce)) (Math|Float|Clamp(Float) (* (- (Variables|Default|GetNatureSuspensionLength) (Variables|Default|GetSuspLength)) (Variables|Default|GetSuspStrength)) 0.0 (LocalVariables|GetTempMaxForce)) (* (/ (- (Variables|Default|GetSuspLength) (Variables|Default|GetLastSuspLength)) (LocalVariables|GetDS)) (Variables|Default|GetSuspensonDamp) -1.0)))