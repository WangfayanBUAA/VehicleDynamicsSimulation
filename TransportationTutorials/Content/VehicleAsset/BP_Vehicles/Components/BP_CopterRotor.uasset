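; Helicopter rotor component that applies flight force to a vehicle body and animates its own spin, driven by calls from outside.
; UpdateRotorForce pushes the body at a point above the rotor, combining world-up lift with doubled horizontal pull along the rotor's tilt.
; UpdateRotorRotation builds a clamped spin speed from power and delta time, rotating around local yaw or pitch to suit differently oriented rotors.
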(event EventBeginPlay)

(event EventTick
  (params (DeltaSeconds :type Float%20%28single-precision%29)))

(fn UpdateRotorForce
  (params (inVehicleBody :type Static%20Mesh%20Component%20Object%20Reference) (inRotorPower :type Float%20%28single-precision%29))
  (bind _self self)
  (bind _returnvalue (Math|Vector|GetUpVector _self))
  (Utilities|FlowControl|Sequence
    (:then_0
      (LocalVariables|SetVehicleBody inVehicleBody)
      (LocalVariables|SetRotor%20Rise%20Force inRotorPower))
    (:then_1
      ;[1 1 1] 旋翼升力位置
      (LocalVariables|SetforceLocation (+ (Transformation|GetWorldLocation self) (* (Math|Vector|GetUpVector self) 1e+02)))
      (Utilities|FlowControl|Sequence
        (:then_0
          ;[1 1 1] 转化成升力向量
          (LocalVariables|SetRaiseForce (* "0, 0,1.000000" (LocalVariables|GetRotor%20Rise%20Force)))
          (bind _output_get (LocalVariables|SetmoveForce (* (Math|Vector|MakeVector (.x _returnvalue) (.y _returnvalue) 0.0) (* (LocalVariables|GetRotor%20Rise%20Force) 2.0))))
          (LocalVariables|SetRotorForce (+ _output_get (LocalVariables|GetRaiseForce))))
        (:then_1
          (Class|PrimitiveComponent|AddForceatLocation (LocalVariables|GetVehicleBody) (LocalVariables|GetRotorForce) (LocalVariables|GetforceLocation) "None"))))))

(fn UpdateRotorRotation
  (params (inDeltaScends :type Float%20%28single-precision%29) (RotorPower :type Float%20%28single-precision%29) (isZ :type Boolean))
  (LocalVariables|SetDS inDeltaScends)
  (Variables|Default|SetRotSpeed (Math|Float|Clamp(Float) (+ (* (- RotorPower 1e+01) (LocalVariables|GetDS) 2e+01) (Variables|Default|GetRotSpeed)) 0.0 2e+03))
  (if isZ
    (Transformation|AddLocalRotation self (Math|Rotator|MakeRotator 0.0 0.0 (* (LocalVariables|GetDS) (Variables|Default|GetRotSpeed) -1.0)) false false)
    (else
      (Transformation|AddLocalRotation self (Math|Rotator|MakeRotator 0.0 (* (LocalVariables|GetDS) (Variables|Default|GetRotSpeed) -1.0) 0.0) false false))))