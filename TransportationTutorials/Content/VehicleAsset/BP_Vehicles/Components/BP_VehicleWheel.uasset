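; Vehicle wheel component that simulates sphere-traced suspension and animates wheel steering and rolling for a parent vehicle body.
; Each suspension update traces down from the wheel's initial body-relative mount, stores length and contact, and repositions the wheel.
; Clamped spring-damper pressure from that length is returned as support force, not applied here.
; Steering yaws mount and wheel; spin follows body velocity at the wheel, decaying when unloaded and undriven unless forced.
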(event EventBeginPlay)

(event EventTick
  (params (DeltaSeconds :type Float%20%28single-precision%29)))

(fn UpdateSuspensionLength
  (params (DeltaSeconds :type Float%20%28single-precision%29))
  (bind _wheelinitreltransf (Variables|Default|GetWheelInitRelTransf))
  (bind _parentvehiclebody (Variables|组件|GetParentVehicleBody))
  (bind _returnvalue (Transformation|GetWorldTransform _parentvehiclebody))
  (bind (_location _rotation) (Math|Transform|BreakTransform _wheelinitreltransf))
  (Variables|SuspensionInfo|SetLastSuspLength (Variables|SuspensionInfo|GetSuspLength))
  (LocalVariables|SetsuspLocation (Math|Transform|TransformLocation _returnvalue _location))
  (LocalVariables|SetSuspDirection (Math|Vector|GetUpVector (Math|Transform|TransformRotation _returnvalue _rotation)))
  (bind (_outhit _returnvalue_2) (Collision|SphereTraceByChannel (LocalVariables|GetsuspLocation) (+ (LocalVariables|GetsuspLocation) (* (LocalVariables|GetSuspDirection) (* (+ (Variables|SuspensionInfo|GetNatureSuspensionLength) 1.0) -1.0))) (Variables|WheelInfos|GetWheelRadius) "TraceTypeQuery3" false 0 "None"))
  (if _returnvalue_2
    (Variables|Default|SetLand%20Impact%20Point (.ImpactPoint (Collision|BreakHitResult _outhit)))
    (Variables|SuspensionInfo|SetSuspLength (- (Math|Vector|VectorLength (- (LocalVariables|GetsuspLocation) (Variables|Default|GetLand%20Impact%20Point))) (Variables|WheelInfos|GetWheelRadius)))
    (Variables|WheelInfos|SetWheel%20Impact%20Normal (.ImpactNormal (Collision|BreakHitResult _outhit)))
    (else
      (Variables|SuspensionInfo|SetSuspLength (Variables|SuspensionInfo|GetNatureSuspensionLength))))
  (Transformation|SetWorldLocation self (+ (LocalVariables|GetsuspLocation) (* (LocalVariables|GetSuspDirection) (* (Variables|SuspensionInfo|GetSuspLength) -1.0))) false false)
  (return))

(fn SetInitInfo
  (params (ParentVehicleBody :type Static%20Mesh%20Component%20Object%20Reference) (WheelInitRelTransf :type Transform) (SuspensonDamp :type Float%20%28single-precision%29) (SuspStrength :type Float%20%28single-precision%29))
  (Variables|组件|SetParentVehicleBody ParentVehicleBody)
  (Variables|Default|SetWheelInitRelTransf WheelInitRelTransf)
  (Variables|SuspensionInfo|SetSuspensonDamp SuspensonDamp)
  (Variables|SuspensionInfo|SetSuspStrength SuspStrength))

(fn IsZeroPressure
  (return (== (- (Variables|SuspensionInfo|GetNatureSuspensionLength) (Variables|SuspensionInfo|GetSuspLength)) 0.0)))

(fn GetPressure
  (params (DeltaSeconds :type Float%20%28single-precision%29))
  (LocalVariables|SetDS DeltaSeconds)
  (LocalVariables|SetTempMaxForce (* (Variables|SuspensionInfo|GetNatureSuspensionLength) (Variables|SuspensionInfo|GetSuspStrength)))
  (return (Math|Float|Clamp(Float) (+ (Math|Float|Clamp(Float) (* (- (Variables|SuspensionInfo|GetNatureSuspensionLength) (Variables|SuspensionInfo|GetSuspLength)) (Variables|SuspensionInfo|GetSuspStrength)) 0.0 (LocalVariables|GetTempMaxForce)) (* (/ (- (Variables|SuspensionInfo|GetSuspLength) (Variables|SuspensionInfo|GetLastSuspLength)) (LocalVariables|GetDS)) (Variables|SuspensionInfo|GetSuspensonDamp) -1.0)) (* (LocalVariables|GetTempMaxForce) -1.0) (LocalVariables|GetTempMaxForce)) (Math|Float|Clamp(Float) (* (- (Variables|SuspensionInfo|GetNatureSuspensionLength) (Variables|SuspensionInfo|GetSuspLength)) (Variables|SuspensionInfo|GetSuspStrength)) 0.0 (LocalVariables|GetTempMaxForce)) (* (/ (- (Variables|SuspensionInfo|GetSuspLength) (Variables|SuspensionInfo|GetLastSuspLength)) (LocalVariables|GetDS)) (Variables|SuspensionInfo|GetSuspensonDamp) -1.0)))

(fn GetSupportVector
  (params (DeltaSeconds :type Float%20%28single-precision%29))
  (bind (_pressure _springforce _dampforce) (CallFunction|GetPressure DeltaSeconds))
  (return _pressure _springforce _dampforce (Math|Transform|TransformDirection (Variables|Default|GetWheelInitRelTransf) (Math|Vector|GetUpVector (.Rotation (Math|Transform|BreakTransform (Variables|Default|GetWheelInitRelTransf)))))))

(fn SetWheelSteerAngle
  (params (inSteerAngle :type Float%20%28single-precision%29))
  (bind _self self)
  (bind _relativerotation (Variables|Default|GetRelativeRotation _self))
  (bind (_roll _pitch) (Math|Rotator|BreakRotator _relativerotation))
  (bind _returnvalue (Math|Vector|GetUpVector _relativerotation))
  (bind _output_get (Variables|Default|SetSteer%20Angle inSteerAngle))
  (Variables|Default|SetWheelInitRelTransf (Math|Transform|MakeTransform (.location (Variables|Default|GetWheelInitRelTransf)) (Math|Rotator|MakeRotator (.Roll (Math|Rotator|BreakRotator (.rotation (Variables|Default|GetWheelInitRelTransf)))) (.Pitch (Math|Rotator|BreakRotator (.rotation (Variables|Default|GetWheelInitRelTransf)))) _output_get) (.scale (Variables|Default|GetWheelInitRelTransf))))
  (if (> (Math|Float|Absolute(Float) (.z _returnvalue)) 0.01)
    (Transformation|SetRelativeRotation self (Math|Rotator|MakeRotator _roll _pitch (+ (Variables|Default|GetSteer%20Angle) (Math|Float|SelectFloat 0.0 1.8e+02 (>= (.z _returnvalue) 0.0)))) false false)))

(fn GetSuspensionRotation
  (return (Math|Transform|TransformRotation (Transformation|GetWorldTransform (Variables|组件|GetParentVehicleBody)) (.rotation (Variables|Default|GetWheelInitRelTransf)))))

(fn WheelRooling
  (params (DeltaSec :type Float%20%28single-precision%29) (ThrottleValue :type Float%20%28single-precision%29) (ForceRolling :type Boolean))
  (Utilities|FlowControl|Sequence
    (:then_0
      (if (Math|Boolean|ORBoolean (not (CallFunction|IsZeroPressure)) (and (> ThrottleValue 0.0) (Variables|WheelInfos|GetisDrivingWheel)) ForceRolling)
        (bind _returnvalue (Class|PrimitiveComponent|GetPhysicsLinearVelocityatPoint (Variables|组件|GetParentVehicleBody) (Transformation|GetWorldLocation) "None"))
        (bind _output_get (LocalVariables|SetSuspensionSpeed (Math|Vector|VectorLengthXY _returnvalue)))
        (bind _output_get_2 (LocalVariables|SetEdge%20Speed (* (Math|Float|Sign(Float) (Math|Vector|DotProduct (Math|Vector|GetForwardVector (Transformation|GetWorldRotation (Variables|组件|GetParentVehicleBody))) _returnvalue)) _output_get)))
        (Variables|Default|SetRotSpeed (* (* -1 (/ _output_get_2 (Variables|WheelInfos|GetWheelRadius))) 57.310001))
        (else
          (Variables|Default|SetRotSpeed (* (Variables|Default|GetRotSpeed) 0.98)))))
    (:then_1
      (Transformation|AddLocalRotation self (Math|Rotator|MakeRotator 0.0 (* (Variables|Default|GetRotSpeed) DeltaSec) 0.0) true true))))