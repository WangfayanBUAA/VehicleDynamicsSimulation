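; A vehicle propeller component that computes thrust and spins itself, driven by calls from outside rather than its own Tick.
; UpdatePropellForce returns a force vector along the component's world forward axis, scaled from the input power.
; PropellerRot rolls the component each call at a rate set by max speed, power percent and delta time, with a flag choosing clockwise or counterclockwise.
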(event EventBeginPlay)

(event EventTick
  (params (DeltaSeconds :type Float%20%28single-precision%29)))

(fn UpdatePropellForce
  (params (DeltaTime :type Float%20%28single-precision%29) (InputPower :type Float%20%28single-precision%29))
  (LocalVariables|SetDS DeltaTime)
  (return (* (Math|Vector|GetForwardVector (Transformation|GetWorldRotation self)) (* InputPower 1e+03))))

(fn PropellerRot
  (params (inDeltaSeconds :type Float%20%28single-precision%29) (inPowerPercent :type Float%20%28single-precision%29))
  (Transformation|AddRelativeRotation self (Math|Rotator|MakeRotator (* (Variables|Default|GetMaxRotSpeed) inPowerPercent inDeltaSeconds (Math|Float|SelectFloat 1.0 -1.0 (Variables|Default|GetisClockwise))) 0.0 0.0) false false))